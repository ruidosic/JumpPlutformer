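; BP_Conrollers is an interactable lever-style control that switches on and off, relaying Open/Close to its linked ActorsToUse and raising game events.
; A timeline lerps the lever pivot between off and on transforms with 3D sounds, blocking interaction while moving.
; UseAfterAnim selects whether state and targets change immediately or when the animation finishes.
; SetupSettings takes struct-based configuration, and an optional trigger box reports player overlap to the player.
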(event `self.Use`
  (params (GameEvent :type Boolean))
  ;[1 1 1] Interact
  (`/Game/Blueprints/Core/BPM_CoreEngine.GE_CheckInteraction`)
  (if (`self.On / Off`)
    (`self.Close/Off` false)
    (else
      (`self.Open/On` false))))

(event `self.Open/On`
  (params (GameEvent :type Boolean))
  (bind _actorstouse (`self.ActorsToUse`))
  ;[1 1 1] Open / Close Settings
  (`/Game/Blueprints/Core/BPM_CoreEngine.GE_CheckInteraction`)
  (if (not (`self.On / Off`))
    (if (not (`self.UseAfterAnim`))
      (set `self.On / Off` true)
      (`self.Open/On` (`self.ActorsToUse`) false)
      (`self.GameEventCheck` "NewEnumerator1"))
    (set `self.InteractionEnabled` false)
    (`/Game/Blueprints/Core/BPM_CoreEngine.GE_3DSound` (`self.HitSound`) false (`self.TurnOnSound`) (`self.LeverPivot`) (`self.Attenuation`))
    (`/Game/Blueprints/Core/BPM_CoreEngine.GE_3DSound` null false (`self.LoopSound`) (`self.LeverPivot`) (`self.Attenuation`))
    (bind (_direction _animation) (`Timeline|LiverTimeline` :!via `PlayFromStart` :!label _label)
      (:`Update`
        (`SceneComponent.K2_SetRelativeLocationAndRotation` (`self.LeverPivot`) (`KismetMathLibrary.VLerp` (`self.OffLocation`) (`self.OnLocation`) _animation) (`KismetMathLibrary.RLerp` (`self.OffRotation`) (`self.OnRotation`) _animation) false false))
      (:`Finished`
        (switch `ETimelineDirection` _direction
          (:`Forward`
            (if (`self.UseAfterAnim`)
              (set `self.On / Off` true)
              (`self.Open/On` _actorstouse false)
              (`self.GameEventCheck` "NewEnumerator1")))
          (:`Backward`
            (if (`self.UseAfterAnim`)
              (set `self.On / Off` false)
              (`self.Close/Off` _actorstouse false)
              (`self.GameEventCheck` "NewEnumerator2"))))
        (set `self.InteractionEnabled` true)
        (if (`self.StopSoundAfterAnimation`)
          (`/Game/Blueprints/Core/BPM_CoreEngine.GE_StopAll3DSound`))
        (`/Game/Blueprints/Core/BPM_CoreEngine.GE_3DSound` null false (`self.HitSound`) (`self.LeverPivot`) (`self.Attenuation`))))))

(event `self.Close/Off`
  (params (GameEvent :type Boolean))
  ;[1 1 1] Open / Close Settings
  (`/Game/Blueprints/Core/BPM_CoreEngine.GE_CheckInteraction`)
  (if (`self.On / Off`)
    (if (not (`self.UseAfterAnim`))
      (set `self.On / Off` false)
      (`self.Close/Off` (`self.ActorsToUse`) false)
      (`self.GameEventCheck` "NewEnumerator2"))
    (set `self.InteractionEnabled` false)
    (`/Game/Blueprints/Core/BPM_CoreEngine.GE_3DSound` (`self.HitSound`) false (`self.TurnOffSound`) (`self.LeverPivot`) (`self.Attenuation`))
    (`/Game/Blueprints/Core/BPM_CoreEngine.GE_3DSound` null false (`self.LoopSound`) (`self.LeverPivot`) (`self.Attenuation`))
    (goto _label :!via `ReverseFromEnd`)))

(event `self.TriggerToUse.OnComponentBeginOverlap`
  (params (OverlappedComponent :type "PrimitiveComponent Object Reference") (OtherActor :type "Actor Object Reference") (OtherComp :type "PrimitiveComponent Object Reference") (OtherBodyIndex :type Integer) (bFromSweep :type Boolean) (SweepResult :type "HitResult Structure (by ref)"))
  ;[1 1 1] Overlap With Player
  (if (`self.UseTrigger`)
    (if (== OtherActor (`GameplayStatics.GetPlayerPawn` 0))
      (bind _as_core_engine (`/Game/Blueprints/Core/BP_Functions.GetPlayer`))
      (`/Game/Blueprints/Core/BP_CoreEngine.UseOverlappedActor` _as_core_engine self))))

(fn `SetupSettings`
  (params (`Trigger Settings` :type "/Game/Blueprints/UsableAssets/Doors/Structs/Struct_TriggerSettings Structure") (`Mesh Settings` :type "/Game/Blueprints/UsableAssets/Controllers/Strtucts/Struct_ControllerMeshSettings Structure") (`Lever Settings` :type "/Game/Blueprints/UsableAssets/Controllers/Strtucts/Struct_ControllerSettings Structure") (`Game Events` :type "Array of /Game/Blueprints/Events/Structs/Struct_GameEvents Structure") (Attenuation :type "SoundAttenuation Object Reference"))
  (bind (_usetrigger _triggersize) (break `/Game/Blueprints/UsableAssets/Doors/Structs/Struct_TriggerSettings` `Trigger Settings`))
  (bind (_leverbasemesh _levermesh) (break `/Game/Blueprints/UsableAssets/Controllers/Strtucts/Struct_ControllerMeshSettings` `Mesh Settings`))
  (bind (_generationinfo _turninfo _useinfo) (break `/Game/Blueprints/UsableAssets/Controllers/Strtucts/Struct_ControllerSettings` `Lever Settings`))
  (bind (_onoff _offlocation _onlocation _offrotation _onrotation) (break `/Game/Blueprints/UsableAssets/Controllers/Strtucts/Struct_ControllerGenerationInfo` _generationinfo))
  (bind (_turnanimationspeedsec _stopsoundafteranim _turnonsound _turnoffsound _hitsound _loopsound) (break `/Game/Blueprints/UsableAssets/Controllers/Strtucts/Struct_ControllerTurnInfo` _turninfo))
  (bind (_actorstouse _useafteranim) (break `/Game/Blueprints/UsableAssets/Controllers/Strtucts/Struct_ControllerUseInfo` _useinfo))
  ;[1 1 1] Setup Attenuation
  (set `self.Attenuation` Attenuation)
  ;[1 1 1] Setup Game Events
  (set `self.GameEvents` `Game Events`)
  ;[1 1 1] Setup Trigger Settings
  (set `self.UseTrigger` _usetrigger)
  (set `self.BoxExtended` _triggersize)
  ;[1 1 1] Setup Mesh Settings
  (set `self.ControlBaseMesh` _leverbasemesh)
  (set `self.ControlMesh` _levermesh)
  ;[1 1 1] Setup Generation Info
  (set `self.On / Off` _onoff)
  (set `self.OffLocation` _offlocation)
  (set `self.OnLocation` _onlocation)
  (set `self.OffRotation` _offrotation)
  (set `self.OnRotation` _onrotation)
  ;[1 1 1] Setup Turn Info
  (set `self.Turn Animation Speed (Sec)` _turnanimationspeedsec)
  (set `self.StopSoundAfterAnimation` _stopsoundafteranim)
  (set `self.TurnOnSound` _turnonsound)
  (set `self.TurnOffSound` _turnoffsound)
  (set `self.HitSound` _hitsound)
  (set `self.LoopSound` _loopsound)
  ;[1 1 1] Setup Use Info
  (set `self.ActorsToUse` _actorstouse)
  (set `self.UseAfterAnim` _useafteranim))

(fn `UserConstructionScript`
  (bind _on___off (`self.On / Off`))
  (`/Game/Blueprints/Core/BP_Functions.SetMesh` (`self.ControlBase`) (`self.ControlBaseMesh`))
  (`/Game/Blueprints/Core/BP_Functions.SetMesh` (`self.Control`) (`self.ControlMesh`))
  (`/Game/Blueprints/Core/BP_Functions.PlayRate` (`self.LiverTimeline`) (`self.Turn Animation Speed (Sec)`))
  (`BoxComponent.SetBoxExtent` (`self.TriggerToUse`) (`self.BoxExtended`) true)
  (`SceneComponent.K2_SetRelativeLocation` (`self.TriggerToUse`) (`KismetMathLibrary.MakeVector` (/ (.x (`self.BoxExtended`)) 10.0) (/ (.y (`self.BoxExtended`)) 10.0) (.z (`self.BoxExtended`))) false false)
  (`SceneComponent.K2_SetRelativeLocationAndRotation` (`self.LeverPivot`) (select `bool` _on___off :`false` (`self.OffLocation`) :`true` (`self.OnLocation`)) (select `bool` _on___off :`false` (`self.OffRotation`) :`true` (`self.OnRotation`)) false false))