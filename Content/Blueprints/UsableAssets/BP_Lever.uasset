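; BP_Lever is a usable lever that toggles linked ActorsToUse on and off and raises game events.
; Use flips the state, and a timeline lerps the pivot between off and on transforms, with 3D sounds and interaction disabled during motion.
; UseAfterAnim defers the state change and linked actions until the animation finishes.
; Its trigger box, sized in the construction script, reports the lever to the overlapping player.
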(event `self.Use`
  (params (GameEvent :type Boolean))
  ;[1 1 1] Interact
  (`/Game/Blueprints/Core/BPM_CoreEngine.GE_CheckInteraction`)
  (if (`self.On / Off`)
    (`self.Close/Off` false)
    (else
      (`self.Open/On` false))))

(event `self.Open/On`
  (params (GameEvent :type Boolean))
  (bind _actorstouse (`self.ActorsToUse`))
  ;[1 1 1] Open / Close Settings
  (`/Game/Blueprints/Core/BPM_CoreEngine.GE_CheckInteraction`)
  (if (not (`self.On / Off`))
    (if (not (`self.UseAfterAnim`))
      (set `self.On / Off` true)
      (`self.Open/On` (`self.ActorsToUse`) false)
      (`self.GameEventCheck` "NewEnumerator1"))
    (set `self.InteractionEnabled` false)
    (`/Game/Blueprints/Core/BPM_CoreEngine.GE_3DSound` (`self.HitSound`) false (`self.TurnOnSound`) (`self.LeverPivot`) (`self.SoundAttenuation`))
    (`/Game/Blueprints/Core/BPM_CoreEngine.GE_3DSound` null false (`self.LoopSound`) (`self.LeverPivot`) (`self.SoundAttenuation`))
    (bind (_direction _animation) (`Timeline|LiverTimeline` :!via `PlayFromStart` :!label _label)
      (:`Update`
        (`SceneComponent.K2_SetRelativeLocationAndRotation` (`self.LeverPivot`) (`KismetMathLibrary.VLerp` (`self.OffLocation`) (`self.OnLocation`) _animation) (`KismetMathLibrary.RLerp` (`self.OffRotation`) (`self.OnRotation`) _animation) false false))
      (:`Finished`
        (switch `ETimelineDirection` _direction
          (:`Forward`
            (if (`self.UseAfterAnim`)
              (set `self.On / Off` true)
              (`self.Open/On` _actorstouse false)
              (`self.GameEventCheck` "NewEnumerator1")))
          (:`Backward`
            (if (`self.UseAfterAnim`)
              (set `self.On / Off` false)
              (`self.Close/Off` _actorstouse false)
              (`self.GameEventCheck` "NewEnumerator2"))))
        (set `self.InteractionEnabled` true)
        (if (`self.StopSoundAfterAnimation`)
          (`/Game/Blueprints/Core/BPM_CoreEngine.GE_StopAll3DSound`))
        (`/Game/Blueprints/Core/BPM_CoreEngine.GE_3DSound` null false (`self.HitSound`) (`self.LeverPivot`) (`self.SoundAttenuation`))))))

(event `self.Close/Off`
  (params (GameEvent :type Boolean))
  ;[1 1 1] Open / Close Settings
  (`/Game/Blueprints/Core/BPM_CoreEngine.GE_CheckInteraction`)
  (if (`self.On / Off`)
    (if (not (`self.UseAfterAnim`))
      (set `self.On / Off` false)
      (`self.Close/Off` (`self.ActorsToUse`) false)
      (`self.GameEventCheck` "NewEnumerator2"))
    (set `self.InteractionEnabled` false)
    (`/Game/Blueprints/Core/BPM_CoreEngine.GE_3DSound` (`self.HitSound`) false (`self.TurnOffSound`) (`self.LeverPivot`) (`self.SoundAttenuation`))
    (`/Game/Blueprints/Core/BPM_CoreEngine.GE_3DSound` null false (`self.LoopSound`) (`self.LeverPivot`) (`self.SoundAttenuation`))
    (goto _label :!via `ReverseFromEnd`)))

(event `self.TriggerToUse.OnComponentBeginOverlap`
  (params (OverlappedComponent :type "PrimitiveComponent Object Reference") (OtherActor :type "Actor Object Reference") (OtherComp :type "PrimitiveComponent Object Reference") (OtherBodyIndex :type Integer) (bFromSweep :type Boolean) (SweepResult :type "HitResult Structure (by ref)"))
  ;[1 1 1] Overlap With Player
  (if (== OtherActor (`GameplayStatics.GetPlayerPawn` 0))
    (bind _as_core_engine (`/Game/Blueprints/Core/BP_Functions.GetPlayer`))
    (`/Game/Blueprints/Core/BP_CoreEngine.UseHitActor` _as_core_engine self)))

(fn `UserConstructionScript`
  (set `self.GameEvents` (`self.CustomGameEvents`))
  (`/Game/Blueprints/Core/BP_Functions.PlayRate` (`self.LiverTimeline`) (`self.Animation Speed (Sec)`))
  (`BoxComponent.SetBoxExtent` (`self.TriggerToUse`) (`self.BoxExtended`) true)
  (`SceneComponent.K2_SetRelativeLocation` (`self.TriggerToUse`) (`KismetMathLibrary.MakeVector` (/ (.x (`self.BoxExtended`)) 10.0) (/ (.y (`self.BoxExtended`)) 10.0) (.z (`self.BoxExtended`))) false false))