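; BP_Inspectable is a usable actor that provides the shared logic for inspecting an item.
; BeginInspection disables player input, registers itself with the player Core, attaches InspectionActor to InspectionPivot, adjusts its shadow casting, plays a sound and shows the interaction widget.
; A timeline blends depth-of-field aperture and calls an empty update event, with stop and reverse controls.
; Construction makes the inspection meshes ignore the Pawn collision channel.
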(event `BeginInspection`
  ;[1 1 1] Begin Inpection
  (`/Game/Blueprints/Core/BP_Functions.PlayerInput` false)
  (bind _as_core_engine (`/Game/Blueprints/Core/BP_Functions.GetPlayer`))
  (bind _output_get (set `self.Core` _as_core_engine))
  (set `/Game/Blueprints/Core/BP_CoreEngine.InteractionItemRef` self _output_get)
  (bind _output_get_2 (set `/Game/Blueprints/Core/BP_CoreEngine.Inspecting` true _output_get))
  (set `self.Inspecting` _output_get_2)
  (set `self.Begin` true)
  (set `self.WorldTransform` (`self.GetTransform`))
  (`self.CastInspectingShadow` (`self.InspectionShadow`))
  (`SceneComponent.K2_AttachToComponent` (`self.InspectionActor`) (`self.InspectionPivot`) "None" "KeepWorld" "SnapToTarget" "SnapToTarget" true)
  (`self.CreateInspectionWidget`)
  (`/Game/Blueprints/Core/BPM_CoreEngine.GE_2DSound` (`self.BeginInspectionSound`) true)
  (`self.PlayInspectionTimeline`))

(event `CreateInspectionWidget`
  ;[1 1 1] Inspection Create / Destroy
  (bind _returnvalue (`|CreateWidget` "/Game/Blueprints/Widgets/Interaction/WBP_Interaction.WBP_Interaction_C"))
  (`UserWidget.AddToViewport` _returnvalue 0))

(event `HideInspectionWidget`
  ;[1 1 1] Inspection Create / Destroy
  (`Widget.RemoveFromParent` (stale `CreateInspectionWidget` _returnvalue)))

(event `PlayInspectionTimeline`
  (bind _core (`self.Core`))
  ;[1 1 1] Inspection Timeline
  (bind (_direction _animation) (`Timeline|InspectionTimeline` :!via `PlayFromStart` :!label _label)
    (:`Update`
      (set `self.AnimationDirection` _direction)
      (set `self.AnimationValue` _animation)
      (set `/Game/Blueprints/Core/BP_CoreEngine.CurrentAperture` (`KismetMathLibrary.Lerp` (`/Game/Blueprints/Core/BP_CoreEngine.DOF Aperature` _core) (`/Game/Blueprints/Core/BP_CoreEngine.DOF Aperature (Inspecting)` _core) _animation) (`self.Core`))
      (`self.UpdateInspectionTimeline`))))

(event `StopInspectionTimeline`
  ;[1 1 1] Inspection Timeline
  (goto _label :!via `Stop`))

(event `ReverseInspectionTimeline`
  (params (`Reverse from Current` :type Boolean))
  ;[1 1 1] Inspection Timeline
  (if `Reverse from Current`
    (goto _label :!via `Reverse`)
    (else
      (goto _label :!via `ReverseFromEnd`))))

(event `UpdateInspectionTimeline`)

(event `FinishedInspectionTimeline`)

(fn `UserConstructionScript`
  (`parent.UserConstructionScript`)
  (for _array_element (`SceneComponent.GetChildrenComponents` (`self.InspectionActor`) true)
    (`/Engine/EditorBlueprintResources/StandardMacros.IsValid` _array_element
      (:`Is Valid`
        (bind _asprimitive_component (cast `PrimitiveComponent` _array_element))
        (`PrimitiveComponent.SetCollisionResponseToChannel` _asprimitive_component "ECC_Pawn" "ECR_Ignore")))))