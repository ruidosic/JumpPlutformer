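; BP_PortalV2 is a portal actor whose mesh displays a render texture through a dynamic material.
; On BeginPlay it sets its target from PortalTarget, then creates a material instance from M_PortalBase_Inst and applies it to PortalMesh.
; SetRTT feeds a valid render texture into the material's Portal parameter, and ClearRTT empties that parameter.
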(event `self.ReceiveBeginPlay`
  (`self.SetTarget` (`self.PortalTarget`))
  (bind _returnvalue (`KismetMaterialLibrary.CreateDynamicMaterialInstance` "/Game/Assets/MeshMat/Portal/M_PortalBase_Inst.M_PortalBase_Inst"))
  (bind _output_get (set `self.MaterialInstance` _returnvalue))
  (`PrimitiveComponent.SetMaterial` (`self.PortalMesh`) 0 _output_get))

(event `self.ClearRTT`
  (`MaterialInstanceDynamic.SetTextureParameterValue` (`self.MaterialInstance`) "Portal" null))

(event `self.SetRTT`
  (params (RenderTexture :type "Texture Object Reference"))
  (`/Engine/EditorBlueprintResources/StandardMacros.IsValid` RenderTexture
    (:`Is Valid`
      (`MaterialInstanceDynamic.SetTextureParameterValue` (`self.MaterialInstance`) "Portal" RenderTexture))))

(fn `UserConstructionScript`)