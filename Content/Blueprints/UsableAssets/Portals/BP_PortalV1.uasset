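; Linked portal actor that shows the view through its TargetPortal and teleports the player and physics objects there.
; A SceneCapture mirrors the player camera behind the target with a clip plane, rendering to the surface material only while the camera faces the portal's front.
; Overlaps moving inward convert transform, velocity and control rotation into the target's space, with a camera cut for the player.
; Construction applies meshes, open/closed collision and a link arrow.
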(event `self.ReceiveBeginPlay`
  (bind (_x _y) (`KismetMathLibrary.BreakVector2D` (`self.RT Resolution`)))
  (if (`self.IsRenderingEnabled`)
    (bind _returnvalue (`KismetRenderingLibrary.CreateRenderTarget2D` (`KismetMathLibrary.FTrunc` _x) (`KismetMathLibrary.FTrunc` _y)))
    (set `self.RenderTarget` _returnvalue)
    (set `SceneCaptureComponent2D.TextureTarget` (`self.RenderTarget`) (`self.PortalSceneCapture`))
    (set `self.MaterialAsset` "/Game/Assets/MeshMat/Portal/M_PortalSimplePlane_Inst.M_PortalSimplePlane_Inst")
    (bind _returnvalue_2 (`PrimitiveComponent.CreateDynamicMaterialInstance` (`self.PortalMeshPlane`) 0 (`self.MaterialAsset`) "None"))
    (set `self.MID_Plane` _returnvalue_2)
    (`MaterialInstanceDynamic.SetTextureParameterValue` (`self.MID_Plane`) "TextureRT" (`self.RenderTarget`))
    (set `SceneCaptureComponent2D.bEnableClipPlane` true (`self.PortalSceneCapture`))
    (if (`self.Open`)
      (`/Game/Blueprints/Core/BPM_CoreEngine.GE_3DSound` null false (`self.AmbientSound`) (`self.PortalMeshPlane`) (`self.SoundAttenuation`)))))

(event `self.ReceiveTick`
  (params (DeltaSeconds :type "Float (single-precision)"))
  (if (`self.IsRenderingEnabled`)
    (bind _output_get (set `self.CameraLocation` (`SceneComponent.K2_GetComponentLocation` (`PlayerCameraManager.TransformComponent` (`GameplayStatics.GetPlayerCameraManager` 0)))))
    (if (>= (`KismetMathLibrary.Dot_VectorVector` (- _output_get (`self.K2_GetActorLocation`)) (`self.GetActorForwardVector`)) 0.0)
      (set `self.IsPSCNeedToUpdate` true)
      (else
        (set `self.IsPSCNeedToUpdate` false)))
    (set `SceneCaptureComponent.bCaptureEveryFrame` (`self.IsPSCNeedToUpdate`) (`self.PortalSceneCapture`))
    (if (`self.IsPSCNeedToUpdate`)
      ;[1 1 1] Like Mirror Creation
      (`/Engine/EditorBlueprintResources/StandardMacros.IsValid` (`self.TargetPortal`)
        (:`Is Valid`
          (set `SceneCaptureComponent2D.ClipPlaneBase` (`self.K2_GetActorLocation` (`self.TargetPortal`)) (`self.PortalSceneCapture`))
          (set `SceneCaptureComponent2D.ClipPlaneNormal` (`self.GetActorForwardVector` (`self.TargetPortal`)) (`self.PortalSceneCapture`))
          (set `self.PortalCaptureLocation` (`self.ConvertLocation` self (`self.TargetPortal`) (`PlayerCameraManager.GetCameraLocation` (`GameplayStatics.GetPlayerCameraManager` 0))))
          (set `self.PortalCaptureRotation` (`self.ConvertRotation` self (`self.TargetPortal`) (`PlayerCameraManager.GetCameraRotation` (`GameplayStatics.GetPlayerCameraManager` 0))))
          (`SceneComponent.K2_SetWorldLocationAndRotation` (`self.PortalSceneCapture`) (`self.PortalCaptureLocation`) (`self.PortalCaptureRotation`) false false))))))

(event `self.ReceiveActorBeginOverlap`
  (params (OtherActor :type "Actor Object Reference"))
  (`self.TeleportOverlap` OtherActor))

(fn `ChangePortalState`
  (params (Open :type Boolean))
  (bind _returnvalue (select `bool` Open :`false` "ECR_Block" :`true` "ECR_Overlap" :!type "ECollisionResponse Enum"))
  (bind _portalmeshplane (`self.PortalMeshPlane`))
  (`PrimitiveComponent.SetCollisionResponseToChannel` _portalmeshplane "ECC_GameTraceChannel1" _returnvalue)
  (`PrimitiveComponent.SetCollisionResponseToChannel` _portalmeshplane "ECC_Pawn" _returnvalue))

(fn `ChangeTransform`
  (params (Transform :type "Transform Structure"))
  (returns (ReturnValue :type "Transform Structure"))
  (bind _targetportal (`self.TargetPortal`))
  (return (`KismetMathLibrary.MakeTransform` (`self.ConvertLocation` self _targetportal (.location Transform)) (`self.ConvertRotation` self _targetportal (.rotation Transform)))))

(fn `ChangeVelocity`
  (params (Velocity :type "Vector Structure"))
  (returns (ReturnValue :type "Vector Structure"))
  (return (* (`self.ConvertDirection` self (`self.TargetPortal`) (`KismetMathLibrary.Normal` Velocity)) (`KismetMathLibrary.VSize` Velocity))))

(fn `ConvertDirection`
  (params (CurrentPortal :type "/Game/Blueprints/UsableAssets/Portals/BP_PortalV1 Object Reference") (TargetPortal :type "/Game/Blueprints/UsableAssets/Portals/BP_PortalV1 Object Reference") (Direction :type "Vector Structure"))
  (returns (ReturnValue :type "Vector Structure"))
  (return (`KismetMathLibrary.TransformDirection` (`self.GetTransform` TargetPortal) (`KismetMathLibrary.MirrorVectorByNormal` (`KismetMathLibrary.MirrorVectorByNormal` (`KismetMathLibrary.InverseTransformDirection` (`self.GetTransform` CurrentPortal) Direction) (1.0 0.0 0.0)) (0.0 1.0 0.0)))))

(fn `ConvertLocation`
  (params (CurrentPortal :type "/Game/Blueprints/UsableAssets/Portals/BP_PortalV1 Object Reference") (TargetPortal :type "/Game/Blueprints/UsableAssets/Portals/BP_PortalV1 Object Reference") (Location :type "Vector Structure"))
  (returns (ReturnValue :type "Vector Structure"))
  (return (`KismetMathLibrary.TransformLocation` (`self.GetTransform` TargetPortal) (`KismetMathLibrary.InverseTransformLocation` (`KismetMathLibrary.MakeTransform` (.location (`self.GetTransform` CurrentPortal)) (.rotation (`self.GetTransform` CurrentPortal)) (`KismetMathLibrary.MakeVector` (* (.x (.scale (`self.GetTransform` CurrentPortal))) -1.0) (* (.y (.scale (`self.GetTransform` CurrentPortal))) -1.0) (.z (.scale (`self.GetTransform` CurrentPortal))))) Location))))

(fn `ConvertRotation`
  (params (CurrentPortal :type "/Game/Blueprints/UsableAssets/Portals/BP_PortalV1 Object Reference") (TargetPortal :type "/Game/Blueprints/UsableAssets/Portals/BP_PortalV1 Object Reference") (Rotation :type "Rotator Structure"))
  (returns (ReturnValue :type "Rotator Structure"))
  (bind (_x _y _z) (`KismetMathLibrary.GetAxes` Rotation))
  (return (`KismetMathLibrary.MakeRotationFromAxes` (`self.ConvertDirection` CurrentPortal TargetPortal _x) (`self.ConvertDirection` CurrentPortal TargetPortal _y) (`self.ConvertDirection` CurrentPortal TargetPortal _z))))

(fn `TeleportOverlap`
  (params (Actor :type "Actor Object Reference"))
  (locals (OverlappingActor :type "Actor Object Reference") (OverlappingPrimitiveComp :type "PrimitiveComponent Object Reference") (ObjectMesh :type "StaticMeshComponent Object Reference"))
  (bind _returnvalue (`GameplayStatics.GetPlayerPawn` 0))
  (bind _objectmesh (`local.ObjectMesh`))
  (bind _returnvalue_2 (`Pawn.GetController` _returnvalue))
  (bind _returnvalue_3 (`Pawn.GetMovementComponent` (`GameplayStatics.GetPlayerPawn` 0)))
  (bind _returnvalue_4 (`self.ChangeVelocity` (`PrimitiveComponent.GetPhysicsAngularVelocityInRadians` (`local.OverlappingPrimitiveComp`) "None")))
  (bind _output_get (set `local.OverlappingActor` Actor))
  (`/Engine/EditorBlueprintResources/StandardMacros.IsValid` _output_get
    (:`Is Valid`
      (if (!= _output_get self)
        (`|ExecutionSequence`
          (:`then_0`
            (if (== (`local.OverlappingActor`) (`GameplayStatics.GetPlayerPawn` 0))
              (`PlayerCameraManager.SetGameCameraCutThisFrame` (`GameplayStatics.GetPlayerCameraManager` 0))))
          (:`then_1`
            (`|ExecutionSequence`
              (:`then_0`
                (if (and (< (`KismetMathLibrary.Dot_VectorVector` (`KismetMathLibrary.Normal` (`self.GetVelocity` (`local.OverlappingActor`))) (`self.GetActorForwardVector`)) 0.0) (> (`KismetMathLibrary.Dot_VectorVector` (`self.GetActorForwardVector`) (- (+ (`self.K2_GetActorLocation` (`local.OverlappingActor`)) (* (`self.GetVelocity` (`local.OverlappingActor`)) (`GameplayStatics.GetWorldDeltaSeconds`))) (`self.K2_GetActorLocation`))) 0.0) (not (`KismetMathLibrary.InRange_FloatFloat` (.z (`self.GetActorForwardVector` (`self.TargetPortal`))) 0.7)))
                  (`|ExecutionSequence` :!label _label
                    (:`then_0`
                      (for _array_element (`self.K2_GetComponentsByClass` (`local.OverlappingActor`) "/Script/Engine.ActorComponent")
                        (bind _asprimitive_component (cast `PrimitiveComponent` _array_element))
                        (bind _output_get_2 (set `local.OverlappingPrimitiveComp` _asprimitive_component))
                        (bind _returnvalue_5 (`PrimitiveComponent.GetPhysicsLinearVelocity` _output_get_2 "None"))
                        (bind _returnvalue_6 (`self.ChangeVelocity` _returnvalue_5))
                        (if (> (`KismetMathLibrary.VSizeSquared` _returnvalue_6) 1.0)
                          (`PrimitiveComponent.SetAllPhysicsLinearVelocity` (`local.OverlappingPrimitiveComp`) (+ _returnvalue_6 (* (`self.GetActorForwardVector`) 10)) false)
                          (if (> (`KismetMathLibrary.VSizeSquared` _returnvalue_4) 1.0)
                            (`PrimitiveComponent.SetAllPhysicsAngularVelocityInRadians` (`local.OverlappingPrimitiveComp`) _returnvalue_4 false)))))
                    (:`then_1`
                      (if (== (`local.OverlappingActor`) (`GameplayStatics.GetPlayerPawn` 0))
                        (`self.K2_SetActorTransform` (`local.OverlappingActor`) (`self.ChangeTransform` (`self.GetTransform` (`local.OverlappingActor`))) false true)
                        (else
                          (`/Engine/EditorBlueprintResources/StandardMacros.IsValid` _objectmesh
                            (:`Is Valid`
                              (`SceneComponent.K2_SetWorldTransform` _objectmesh (`self.ChangeTransform` (`SceneComponent.K2_GetComponentToWorld` _objectmesh)) false true)
                              (`self.GameEventCheck` "NewEnumerator22"))))))
                    (:`then_2`
                      (if (== (`local.OverlappingActor`) _returnvalue)
                        (`Controller.SetControlRotation` _returnvalue_2 (`self.ConvertRotation` self (`self.TargetPortal`) (`Controller.GetControlRotation` _returnvalue_2)))
                        (set `MovementComponent.Velocity` (`self.ChangeVelocity` (`MovementComponent.Velocity` _returnvalue_3)) _returnvalue_3)
                        (message `/Game/Blueprints/UsableAssets/Portals/BPI_Portal.OnLandedRotation` (`GameplayStatics.GetPlayerPawn` 0) self (`self.TargetPortal`))
                        (`self.GameEventCheck` "NewEnumerator25")))
                    (:`then_3`))))
              (:`then_1`
                (bind _asbp_physics_object (cast `/Game/Blueprints/UsableAssets/PhysicsObjects/BP_PhysicsObject` (`local.OverlappingActor`))) ; Check that Actor is Physics
                ;[1 1 1] Check physics move into portal
                (bind _output_get_3 (set `local.ObjectMesh` (`/Game/Blueprints/UsableAssets/PhysicsObjects/BP_PhysicsObject.ObjectMesh` _asbp_physics_object)))
                (bind _returnvalue_7 (`PrimitiveComponent.GetPhysicsLinearVelocity` _output_get_3 "None"))
                (if (< (`KismetMathLibrary.Dot_VectorVector` _returnvalue_7 (`self.GetActorForwardVector`)) 0.0)
                  (goto _label))))))))))

(fn `UserConstructionScript`
  (bind _portalsurfacesize (`self.PortalSurfaceSize`))
  (bind (_portalmeshplane _portalmeshframe) (break `/Game/Blueprints/UsableAssets/Portals/Struct_PortalMesh` (`self.PortalMesh`)))
  (bind _returnvalue (- (`self.K2_GetActorLocation` (`self.TargetPortal`)) (`self.K2_GetActorLocation`)))
  (bind _returnvalue_2 (`KismetMathLibrary.Cross_VectorVector` _returnvalue (0.0 0.0 1.0)))
  (`/Game/Blueprints/Core/BP_Functions.SetMesh` (`self.PortalMeshPlane`) _portalmeshplane)
  (`/Game/Blueprints/Core/BP_Functions.SetMesh` (`self.PortalMeshFrame`) _portalmeshframe)
  (`SceneComponent.SetRelativeScale3D` (`self.PortalMeshPlane`) _portalsurfacesize)
  (`SceneComponent.SetRelativeScale3D` (`self.PortalMeshFrame`) (* _portalsurfacesize 0.01))
  (`self.ChangePortalState` (`self.Open`))
  (`/Engine/EditorBlueprintResources/StandardMacros.IsValid` (`self.TargetPortal`)
    (:`Is Valid`
      (bind _returnvalue_3 (`AddComponent|NODE_AddArrowComponent-0`))
      (`SceneComponent.K2_SetWorldTransform` _returnvalue_3 (`KismetMathLibrary.MakeTransform` (`self.K2_GetActorLocation`) (`KismetMathLibrary.MakeRotationFromAxes` _returnvalue _returnvalue_2 (`KismetMathLibrary.Cross_VectorVector` _returnvalue_2 _returnvalue)) (`KismetMathLibrary.MakeVector` (/ (`KismetMathLibrary.VSize` _returnvalue) (`self.ConnectedArrowDistance`)) 1.0 1.0)) false false)
      (`ArrowComponent.SetArrowColor` _returnvalue_3 (`self.ConnectedArrowColor`)))))