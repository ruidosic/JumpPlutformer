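; BP_SimplePortal is a placeable portal Blueprint that applies its exposed settings at construction time.
; The construction script runs a setup step before calling the parent construction script.
; That step passes surface mesh size, render enable, open state and target portal through setter functions.
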(fn `UserConstructionScript`
  (`self.SetMeshSurfaceSize` (`self.SurfaceMeshSize`))
  (`self.SetIsRenderEnable` (`self.RenderEnable`))
  (`self.SetIsOpen` (`self.Open`))
  (`self.SetTarget` (`self.Target Portal`))
  (`parent.UserConstructionScript`))