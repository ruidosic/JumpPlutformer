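; BP_Keycard is an inventory keycard pickup that operates compatible BP_KeycardControl panels.
; Taking it, via use or inspection, notifies its panels, flags admin access for admin keys and shows a notice.
; Using it from inventory toggles a compatible targeted panel open or closed, or triggers a denied response.
; The construction script maps keycard settings into parent setup, and CheckUnlocked can remove the card once all its panels are open.
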(event `self.Use`
  (params (GameEvent :type Boolean))
  ;[1 1 1] Use Events
  (if (`self.Takeable`)
    (`self.Take` false :!label _label)
    (`KismetSystemLibrary.Delay` 0.01)
    (`self.TakeKey` (`self.CompatibleControlPanel`) false)
    (if (`self.AdminKey`)
      (`/Game/Blueprints/UsableAssets/Electronics/BP_KeycardControl.TakeAdminKey` (`self.CompatibleControlPanel`)))
    (`/Game/Blueprints/Core/BP_Functions.Notice` "" (`self.ItemName`) "added to inventory.")
    (else
      (`self.AlternativeUse` GameEvent))))

(event `self.InspectionUse`
  ;[1 1 1] Use Events
  (if (`self.Takeable`)
    (goto _label)))

(event `self.InventoryUse`
  ;[1 1 1] Use Events
  (bind _as_core_engine (`/Game/Blueprints/Core/BP_Functions.GetPlayer`))
  (if (`|EnumEquality` (`/Game/Blueprints/Core/BP_CoreEngine.InventoryFilter` _as_core_engine) "NewEnumerator3")
    (if (`KismetArrayLibrary.Array_Contains` (`self.CompatibleControlPanel`) (cast `/Game/Blueprints/UsableAssets/Electronics/BP_KeycardControl` (`/Game/Blueprints/Core/BP_CoreEngine.UsableRef` _as_core_engine) :!pure true))
      (bind _as_core_engine_2 (`/Game/Blueprints/Core/BP_Functions.GetPlayer`))
      (bind _asbp_keycard_control (cast `/Game/Blueprints/UsableAssets/Electronics/BP_KeycardControl` (`/Game/Blueprints/Core/BP_CoreEngine.UsableRef` _as_core_engine_2)))
      (if (`/Game/Blueprints/UsableAssets/Electronics/BP_KeycardControl.Open` _asbp_keycard_control)
        (`self.Close/Off` _asbp_keycard_control false)
        (else
          (`self.Open/On` false)))
      (else
        (`/Game/Blueprints/Core/BP_Functions.Notice` "" (`self.ItemName`) "is not compatible.")
        (bind _as_core_engine_3 (`/Game/Blueprints/Core/BP_Functions.GetPlayer`))
        (bind _asbp_keycard_control_2 (cast `/Game/Blueprints/UsableAssets/Electronics/BP_KeycardControl` (`/Game/Blueprints/Core/BP_CoreEngine.UsableRef` _as_core_engine_3)))
        (`/Game/Blueprints/UsableAssets/Electronics/BP_KeycardControl.Denied` _asbp_keycard_control_2)))
    (`self.CloseInventory` (`/Game/Blueprints/Widgets/Interaction/WBP_Interaction.InteractionItemRef` (`/Game/Blueprints/Core/BP_CoreEngine.InteractionWidgetRef` _as_core_engine)))
    (`/Game/Blueprints/Core/BPM_CoreEngine.GE_2DSound` (`self.InteractionSound`) true)))

(event `self.CheckUnlocked`
  ;[1 1 1] Check Unlocked
  (if (`self.RemoveAfterUnlock`)
    (`KismetArrayLibrary.Array_Clear` (`self.AllUnlocked`))
    (for _array_element (`self.CompatibleControlPanel`)
      (`KismetArrayLibrary.Array_Add` (`self.AllUnlocked`) (`/Game/Blueprints/UsableAssets/Electronics/BP_KeycardControl.Open` _array_element)))
    (if (`KismetArrayLibrary.Array_Contains` (`self.AllUnlocked`))
      (`KismetArrayLibrary.Array_Clear` (`self.AllUnlocked`))
      (else
        (`self.RemoveFromInventory`)
        (`self.CloseInventory`)))))

(fn `UserConstructionScript`
  (bind (_adminkey _compatiblecontrolpanels _removeafterunlock) (break `/Game/Assets/MeshMat/Keycard/Struct_KeycardSettings` (`self.KeycardSettings`)))
  (set `self.AdminKey` _adminkey)
  (set `self.CompatibleControlPanel` _compatiblecontrolpanels)
  (`self.SetupSettings` (`self.TriggerSettings`) (`self.KeycardMesh`) (make `/Game/Blueprints/UsableAssets/Inventory/Keys/Struct_KeySettings` (`|MakeArray` null :!type "/Game/Blueprints/Core/BP_Use Object Reference") _removeafterunlock) (`self.Inspection Settings`) (`self.Inventory Settings`) (`self.CreateGameEvents`))
  (`parent.UserConstructionScript`))