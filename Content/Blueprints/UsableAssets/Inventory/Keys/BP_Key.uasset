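; Inspectable inventory key that locks and unlocks its compatible doors.
; It is picked up through use, inspection or an optional player-overlap trigger, then calls TakeKey on each compatible actor.
; Using it from the inventory checks the player's targeted actor against that list, toggles a BP_Door's lock and shows notices.
; CheckUnlocked can remove the key once no compatible door remains locked, and SetupSettings applies configuration from passed-in structs.
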(event `self.AlternativeUse`
  (params (GameEvent :type Boolean))
  ;[1 1 1] Inspection
  (if (not GameEvent)
    (`self.BeginInspection`)))

(event `self.InspectionAlternativeUse`
  ;[1 1 1] Inspection
  (`self.EndInspection` false))

(event `self.InspectionUse`
  ;[1 1 1] Use Events
  (if (`self.Takeable`)
    (`self.Take` false :!label _label)
    (`KismetSystemLibrary.Delay` 0.01)
    (if (`KismetSystemLibrary.IsValid` (stale _array_element))
      (for _array_element (`self.CompatibleActors`)
        (`self.TakeKey` _array_element false) ; this function execute in BP_Door
        (`/Game/Blueprints/Core/BP_Functions.Notice` "" (`self.ItemName`) "added to inventory." :!label _label_2))
      (else
        (goto _label_2)))))

(event `self.Use`
  (params (GameEvent :type Boolean))
  ;[1 1 1] Use Events
  (if (`self.Takeable`)
    (goto _label)
    (else
      (`self.AlternativeUse` GameEvent))))

(event `self.TriggerForUse.OnComponentBeginOverlap`
  (params (OverlappedComponent :type "PrimitiveComponent Object Reference") (OtherActor :type "Actor Object Reference") (OtherComp :type "PrimitiveComponent Object Reference") (OtherBodyIndex :type Integer) (bFromSweep :type Boolean) (SweepResult :type "HitResult Structure (by ref)"))
  ;[1 1 1] Use Events
  ;;[1 1 1] Event Use On Trigger
  (if (and (`self.UseTrigger`) (== OtherActor (`GameplayStatics.GetPlayerPawn` 0)))
    (bind _as_core_engine (`/Game/Blueprints/Core/BP_Functions.GetPlayer`))
    (`/Game/Blueprints/Core/BP_CoreEngine.UseOverlappedActor` _as_core_engine self)))

(event `self.InventoryUse`
  ;[1 1 1] Use Events
  (bind _as_core_engine (`/Game/Blueprints/Core/BP_Functions.GetPlayer` :!label _label_3))
  (if (`|EnumEquality` (`/Game/Blueprints/Core/BP_CoreEngine.InventoryFilter` _as_core_engine) "NewEnumerator2")
    (if (`KismetArrayLibrary.Array_Contains` (`self.CompatibleActors`) (`/Game/Blueprints/Core/BP_CoreEngine.UsableRef` _as_core_engine))
      (`self.Lock/Unlock`)
      (`self.CloseInventory` (`/Game/Blueprints/Widgets/Interaction/WBP_Interaction.InteractionItemRef` (`/Game/Blueprints/Core/BP_CoreEngine.InteractionWidgetRef` _as_core_engine)))
      (`/Game/Blueprints/Core/BPM_CoreEngine.GE_2DSound` (`self.InteractionSound`) true)
      (else
        (`/Game/Blueprints/Core/BP_Functions.Notice` "" "" "doesn't fit.")))))

(event `UseMessage`
  ;[1 1 1] Use Events
  (goto _label_3))

(fn `CheckUnlocked`
  (if (`self.RemoveAfterUnlock`)
    (`KismetArrayLibrary.Array_Clear` (`self.AllUnlocked`))
    (for _array_element (`self.CompatibleActors`)
      (bind _asbp_door (cast `/Game/Blueprints/UsableAssets/Doors/BP_Door` _array_element))
      (`KismetArrayLibrary.Array_Add` (`self.AllUnlocked`) (`/Game/Blueprints/UsableAssets/Doors/BP_Door.Locked` _asbp_door)))
    (if (`KismetArrayLibrary.Array_Contains` (`self.AllUnlocked`) true)
      (`KismetArrayLibrary.Array_Clear` (`self.AllUnlocked`))
      (else
        (`self.RemoveFromInventory`)
        (`self.CloseInventory`)))))

(fn `SetupSettings`
  (params (`Trigger Settings` :type "/Game/Blueprints/UsableAssets/Doors/Structs/Struct_TriggerSettings Structure") (`Mesh Settings` :type "/Game/Blueprints/UsableAssets/Structs/Struct_SetMesh Structure") (`Key Settings` :type "/Game/Blueprints/UsableAssets/Inventory/Keys/Struct_KeySettings Structure") (`Inspection Settings` :type "/Game/Blueprints/UsableAssets/Structs/Struct_InspectionSettings Structure") (`Inventory Settings` :type "/Game/Blueprints/UsableAssets/Structs/Struct_InventorySettings Structure") (`Game Events` :type "Array of /Game/Blueprints/Events/Structs/Struct_GameEvents Structure"))
  (bind (_usetrigger _triggersize) (break `/Game/Blueprints/UsableAssets/Doors/Structs/Struct_TriggerSettings` `Trigger Settings`))
  (bind (_compatibleactors _removeafterunlock) (break `/Game/Blueprints/UsableAssets/Inventory/Keys/Struct_KeySettings` `Key Settings`))
  ;[1 1 1] Setup Trigger Settings
  (set `self.UseTrigger` _usetrigger)
  (set `self.TriggerSize` _triggersize)
  ;[1 1 1] Setup Mesh Settings
  (set `self.KeyMesh` `Mesh Settings`)
  ;[1 1 1] Setup Key Settings
  (set `self.CompatibleActors` _compatibleactors)
  (set `self.RemoveAfterUnlock` _removeafterunlock)
  ;[1 1 1] Setup Inspection and Inventory Settings
  (`self.SetInspection` `Inspection Settings`)
  (`self.SetInventory` `Inventory Settings`)
  ;[1 1 1] Setup Game Events
  (set `self.GameEvents` `Game Events`))

(fn `UserConstructionScript`
  (`parent.UserConstructionScript`)
  (`/Game/Blueprints/Core/BP_Functions.SetMesh` (`self.Key`) (`self.KeyMesh`))
  (`BoxComponent.SetBoxExtent` (`self.TriggerForUse`) (`self.TriggerSize`) true))