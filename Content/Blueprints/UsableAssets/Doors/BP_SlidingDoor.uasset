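; Sliding door Blueprint, a child of a shared door parent, that slides open and closed with handle animation, 3D sounds and game event checks.
; Interaction turns the handle before opening, plays a forced-handle animation when locked, or toggles an open door.
; Three timelines lerp door location and handle rotation; closing resets the handle and can lock the door.
; Construction passes settings to the parent, sets timeline rates and initial pose, and attaches the lock to the handle.
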(event `self.ToggleDoor`
  ;[1 1 1] Toggle / Open / Close Door
  (switch `ETimelineDirection` (stale `self.OpenDoor` _direction)
    (:`Forward`
      (`self.CloseDoor` false))
    (:`Backward`
      (`self.OpenDoor`))))

(event `self.OpenDoor`
  ;[1 1 1] Toggle / Open / Close Door
  (`/Game/Blueprints/Core/BPM_CoreEngine.GE_3DSound` (`self.DoorCloseSound`) false (`self.DoorOpenSound`) (`self.HandlePivot`) (`self.SoundAttenuation`))
  (bind (_direction _animation) (`Timeline|Open/CloseTimeline` :!label _label)
    (:`Update`
      (`SceneComponent.K2_SetRelativeLocation` (`self.DoorPivot`) (`KismetMathLibrary.VLerp` (`self.DoorCloseLocation`) (`self.DoorOpenLocation`) _animation) false false))
    (:`Finished`
      (`/Game/Blueprints/Core/BPM_CoreEngine.GE_Stop3DSound ` (`self.DoorOpenSound`))
      (`/Game/Blueprints/Core/BPM_CoreEngine.GE_Stop3DSound ` (`self.DoorCloseSound`)))
    (:`OpenCloseCheck`
      (switch `ETimelineDirection` _direction
        (:`Forward`
          (set `self.Open` true)
          (`self.GameEventCheck` "NewEnumerator1"))
        (:`Backward`
          (set `self.Open` false)
          (`/Game/Blueprints/Core/BPM_CoreEngine.GE_3DSound` null false (`self.CloseHitSound`) (`self.HandlePivot`) (`self.SoundAttenuation`))
          (`self.ResetHandle`)
          (`self.GameEventCheck` "NewEnumerator2")
          (if (stale `self.CloseDoor` Lock)
            (`self.LockDoor`)))))))

(event `self.CloseDoor`
  (params (Lock :type Boolean))
  ;[1 1 1] Toggle / Open / Close Door
  (`/Game/Blueprints/Core/BPM_CoreEngine.GE_3DSound` (`self.DoorOpenSound`) false (`self.DoorCloseSound`) (`self.HandlePivot`) (`self.SoundAttenuation`))
  (goto _label :!via `Reverse`))

(event `self.OpenHandle`
  ;[1 1 1] Handle Settings
  (bind (_direction _animation) (`Timeline|SlidingHandleTimeline` :!label _label_2)
    (:`Update`
      (`SceneComponent.K2_SetRelativeRotation` (`self.HandlePivot`) (`KismetMathLibrary.RLerp` (`self.HandleReleaseRotation`) (`self.HandleOpenRotation`) _animation) false false))
    (:`Finished`
      (switch `ETimelineDirection` _direction
        (:`Forward`
          (if (`self.Locked`)
            (`self.ForceDoor`)
            (else
              (`self.OpenDoor`))))))
    (:`HandleOpenSound`
      (`/Game/Blueprints/Core/BPM_CoreEngine.GE_3DSound` null false (`self.HandleOpenSound`) (`self.HandlePivot`) (`self.SoundAttenuation`)))
    (:`HandleReleaseSound`
      (`/Game/Blueprints/Core/BPM_CoreEngine.GE_3DSound` null false (`self.HandleReleaseSound`) (`self.HandlePivot`) (`self.SoundAttenuation`)))))

(event `self.ResetHandle`
  ;[1 1 1] Handle Settings
  (goto _label_2 :!via `ReverseFromEnd`))

(event `self.ForceDoor`
  (bind _handleopensound (`self.HandleOpenSound`))
  ;[1 1 1] Force Settings
  (bind (_direction _animation) (`Timeline|SlidingForceTimeline` :!via `PlayFromStart`)
    (:`Update`
      (`SceneComponent.K2_SetRelativeRotation` (`self.HandlePivot`) (`KismetMathLibrary.RLerp` (`self.HandleReleaseRotation`) (`self.ForceRotation`) _animation) false false)
      (`self.GameEventCheck` "NewEnumerator11"))
    (:`ForceSound`
      (`/Game/Blueprints/Core/BPM_CoreEngine.GE_3DSound` _handleopensound false _handleopensound (`self.HandlePivot`) (`self.SoundAttenuation`)))))

(event `self.Open/On`
  (params (GameEvent :type Boolean))
  ;[1 1 1] Open / On
  (`/Game/Blueprints/Core/BPM_CoreEngine.GE_CheckInteraction`)
  (if (`self.Open`)
    (`self.ToggleDoor`)
    (elif (`self.Locked`)
      (`self.ForceDoor`)
      (else
        (`self.OpenHandle`)))))

(fn `UserConstructionScript`
  (bind (_doorinfo _handleinfo _lockinfo _forceinfo _keyinfo) (break `/Game/Blueprints/UsableAssets/Doors/Structs/SlidingDoor/Struct_SlidingDoorSettings` (`self.DoorSettings`)))
  (bind (_doorname _open _dooropenclosedurationsec _knockknocksound _dooropenlocation _doorcloselocation _closehitsound _creaksound _dooropensound _doorclosesound) (break `/Game/Blueprints/UsableAssets/Doors/Structs/SlidingDoor/Struct_SlidingDoorInfo` _doorinfo))
  ;[1 0 0] When we add additional variables in our data structure we must do all this things
  (set `self.DoorOpenLocation` _dooropenlocation)
  (set `self.DoorCloseLocation` _doorcloselocation)
  (set `self.DoorOpenSound` _dooropensound)
  (set `self.DoorCloseSound` _doorclosesound)
  (`self.SetupSettings` (`self.TriggerSettings`) (`self.MeshSettings`) (make `/Game/Blueprints/UsableAssets/Doors/Structs/Struct_DoorSettings` (make `/Game/Blueprints/UsableAssets/Doors/Structs/Struct_DoorInfo` _doorname _open _dooropenclosedurationsec _knockknocksound (struct) (struct) _closehitsound _creaksound) _handleinfo _lockinfo _forceinfo _keyinfo) (`self.CreateGameEvents`) (`self.SoundAttenuation`)) ; Setup Parent Variables
  (`parent.UserConstructionScript`) ; Initialize Parent Configurations
  ;[1 1 1] Initialize that BP Configurations
  (`/Game/Blueprints/Core/BP_Functions.PlayRate` (`self.Open/CloseTimeline`) (`self.Door Open / Close Duration (Sec)`))
  (`/Game/Blueprints/Core/BP_Functions.PlayRate` (`self.SlidingHandleTimeline`) (`self.Handle Open / Release Duration (Sec)`))
  (`/Game/Blueprints/Core/BP_Functions.PlayRate` (`self.SlidingForceTimeline`) (`self.ForceDuration (Sec)`))
  (`SceneComponent.K2_SetRelativeLocation` (`self.DoorPivot`) (select `bool` (`self.Open`) :`false` (`self.DoorCloseLocation`) :`true` (`self.DoorOpenLocation`)) false false)
  (`SceneComponent.K2_SetRelativeRotation` (`self.HandlePivot`) (select `bool` (`self.Open`) :`false` (`self.HandleReleaseRotation`) :`true` (`self.HandleOpenRotation`)) false false)
  (`TimelineComponent.SetNewTime` (`self.Open/CloseTimeline`) (select `bool` (`self.Open`) :`true` 1.0 :!type "Float (single-precision)"))
  (`SceneComponent.K2_AttachToComponent` (`self.LockPivot`) (`self.HandlePivot`) "None" "KeepWorld" "KeepWorld" "SnapToTarget" true))