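; Base physics prop the player can pick up with Alternative Use, carry, drop, or throw along the camera's forward vector.
; A PhysicsHandle follows a timeline-eased HeldSlot on Tick, auto-releasing beyond ReleaseDistance.
; Pawn collision changes while held and returns to Block once the player's overlap ends after release.
; Construction applies physics and sound settings; impacts play force-scaled sounds, game-event checks accompany actions, and children can override Throwed.
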(event `InputAction|AlternativeUse`
  (params (Key :type "Key Structure"))
  ;[1 1 1] Alternative Use
  (:`Pressed`
    (`self.ReleaseObject`)))

(event `self.AlternativeUse`
  (params (GameEvent :type Boolean))
  ;[1 1 1] Alternative Use
  (`self.HeldObject`))

(event `InputAction|Use`
  (params (Key :type "Key Structure"))
  ;[1 1 1] Alternative Use
  (:`Pressed`
    (`self.ReleaseObject`)
    (`self.ThrowObject`)))

(event `HeldObject`
  ;[1 1 1] Held / Release Events
  (`/Game/Blueprints/Core/BPM_CoreEngine.GE_CheckInteraction`)
  (set `self.InteractionEnabled` false)
  (set `self.Carrying` false)
  (`self.SetActorTickEnabled` true)
  (`SceneComponent.K2_SetWorldLocation` (`self.HeldSlot`) (`SceneComponent.K2_GetComponentLocation` (`self.ObjectMesh`)) false false)
  (`PrimitiveComponent.SetSimulatePhysics` (`self.ObjectMesh`) true)
  (`PhysicsHandleComponent.GrabComponentAtLocationWithRotation` (`self.PhysicsHandle`) (`self.ObjectMesh`) "None" (`PrimitiveComponent.GetCenterOfMass` (`self.ObjectMesh`) "None") (`SceneComponent.K2_GetComponentRotation` (`self.HeldSlot`)))
  (`PrimitiveComponent.SetCollisionResponseToChannel` (`self.ObjectMesh`) "ECC_Pawn" (select `bool` (`self.IgnorePawnWhileCarrying`) :`false` "ECR_Block" :`true` "ECR_Ignore" :!type "ECollisionResponse Enum"))
  (`self.ControllerInput` true)
  (bind (_direction _animation) (`Timeline|HeldingTimeline` :!via `PlayFromStart`)
    (:`Update`
      (`SceneComponent.K2_SetRelativeLocation` (`self.HeldSlot`) (`KismetMathLibrary.VLerp` (`SceneComponent.RelativeLocation` (`self.HeldSlot`)) (`self.HeldLocation`) _animation) false false)
      (`self.GameEventCheck` "NewEnumerator19"))
    (:`Finished`
      (set `self.InteractionEnabled` true))))

(event `ReleaseObject`
  (bind _physicshandle (`self.PhysicsHandle`))
  ;[1 1 1] Held / Release Events
  (`/Game/Blueprints/Core/BPM_CoreEngine.GE_CheckInteraction`)
  (`/Engine/EditorBlueprintResources/StandardMacros.IsValid` _physicshandle
    (:`Is Valid`
      (`PhysicsHandleComponent.ReleaseComponent` _physicshandle)
      (`self.SetActorTickEnabled` false)
      (`self.ControllerInput` false)
      (bind _as_core_engine (`/Game/Blueprints/Core/BP_Functions.GetPlayer`))
      (set `/Game/Blueprints/Core/BP_CoreEngine.Helding` false _as_core_engine)
      (set `self.Carrying` false)
      (`PrimitiveComponent.SetCollisionResponseToChannel` (`self.ObjectMesh`) "ECC_Pawn" "ECR_Overlap")
      (`self.GameEventCheck` "NewEnumerator20"))))

(event `ThrowObject`
  ;[1 1 1] Throw Events
  (`/Game/Blueprints/Core/BPM_CoreEngine.GE_CheckInteraction`)
  (`PrimitiveComponent.SetSimulatePhysics` (`self.ObjectMesh`) true)
  (set `self.SoundCooldown` true)
  (bind _as_core_engine (`/Game/Blueprints/Core/BP_Functions.GetPlayer`))
  (`PrimitiveComponent.AddImpulse` (`self.ObjectMesh`) (* (`SceneComponent.GetForwardVector` (`/Game/Blueprints/Core/BP_CoreEngine.PlayerCamera` _as_core_engine)) (`self.ThrowForce`)) "None" false)
  (`self.GameEventCheck` "NewEnumerator21")
  (`self.Throwed`))

(event `self.ReceiveTick`
  (params (DeltaSeconds :type "Float (single-precision)"))
  (bind _heldslot (`self.HeldSlot`))
  ;[1 1 1] Event Tick
  (`PhysicsHandleComponent.SetTargetLocationAndRotation` (`self.PhysicsHandle`) (`SceneComponent.K2_GetComponentLocation` _heldslot) (`SceneComponent.K2_GetComponentRotation` _heldslot))
  (bind _as_core_engine (`/Game/Blueprints/Core/BP_Functions.GetPlayer`))
  (if (> (`KismetMathLibrary.VSize` (- (`self.K2_GetActorLocation` _as_core_engine) (`SceneComponent.K2_GetComponentLocation` (`self.ObjectMesh`)))) (`self.ReleaseDistance`))
    (`self.ReleaseObject`)))

(event `Throwed`
  ;[1 1 1] Throw Events
)

(event `self.ObjectMesh.OnComponentHit`
  (params (HitComponent :type "PrimitiveComponent Object Reference") (OtherActor :type "Actor Object Reference") (OtherComp :type "PrimitiveComponent Object Reference") (NormalImpulse :type "Vector Structure") (Hit :type "HitResult Structure (by ref)"))
  (bind _returnvalue (`KismetMathLibrary.VSize` NormalImpulse))
  (bind _mass (`self.Mass`))
  ;[1 1 1] Hit Sounds Settings
  (`PrimitiveComponent.SetSimulatePhysics` (`self.ObjectMesh`) true)
  (if (and (> _returnvalue (* _mass (`self.HitSoundThreshold`))) (`self.UseHitSound`) (`self.SoundCooldown`))
    (set `self.SoundCooldown` false)
    (`GameplayStatics.SpawnSoundAtLocation` (`self.Hit Sound`) (`SceneComponent.K2_GetComponentLocation` HitComponent) (struct) (`KismetMathLibrary.MapRangeClamped` _returnvalue (* _mass 100.0) 10000.0 (`self.HitSoundMinVolume`) (`self.HitSoundMaxVolume`)) 1.0 0.0 (`self.Attenuation`) null)
    (`KismetSystemLibrary.Delay` 0.25)
    (set `self.SoundCooldown` true)))

(event `self.ObjectMesh.OnComponentEndOverlap`
  (params (OverlappedComponent :type "PrimitiveComponent Object Reference") (OtherActor :type "Actor Object Reference") (OtherComp :type "PrimitiveComponent Object Reference") (OtherBodyIndex :type Integer))
  (if (and (not (`self.Carrying`)) (== OtherActor (`GameplayStatics.GetPlayerPawn` 0)))
    (`PrimitiveComponent.SetCollisionResponseToChannel` (`self.ObjectMesh`) "ECC_Pawn" "ECR_Block")))

(fn `SetupSettings`
  (params (ObjectMesh :type "/Game/Blueprints/UsableAssets/Structs/Struct_SetMesh Structure") (ObjectSettings :type "/Game/Blueprints/UsableAssets/PhysicsObjects/Struct_PhysicsObjectSettings Structure") (GameEvents :type "Array of /Game/Blueprints/Events/Structs/Struct_GameEvents Structure"))
  (bind (_physicssettings _soundsettings) (break `/Game/Blueprints/UsableAssets/PhysicsObjects/Struct_PhysicsObjectSettings` ObjectSettings))
  (bind (_simulatephysics _mass _lineardamping _angulardamping _enablegravity _throwforce _ignorepawnwhilecarrying _heldlocation _releasedistance) (break `/Game/Blueprints/UsableAssets/PhysicsObjects/Struct_POS_Physics` _physicssettings))
  (bind (_usehitsound _hitsound _hitsoundthreshold _hitsoundminvolume _hitsoundmaxvolume _hitsoundattenuation) (break `/Game/Blueprints/UsableAssets/PhysicsObjects/Struct_POS_HitSoundSound` _soundsettings))
  (`/Game/Blueprints/Core/BP_Functions.SetMesh` (`self.ObjectMesh`) ObjectMesh)
  ;[1 1 1] Setup Game Events
  (set `self.GameEvents` GameEvents)
  ;[1 1 1] Setup Physics Settings
  (set `self.SimulatePhysics` _simulatephysics)
  (set `self.Mass` _mass)
  (set `self.LinearDamping` _lineardamping)
  (set `self.AngularDamping` _angulardamping)
  (set `self.EnableGravity` _enablegravity)
  (set `self.ThrowForce` _throwforce)
  (set `self.IgnorePawnWhileCarrying` _ignorepawnwhilecarrying)
  (set `self.HeldLocation` _heldlocation)
  (set `self.ReleaseDistance` _releasedistance)
  ;[1 1 1] Hit Sound Settings
  (set `self.UseHitSound` _usehitsound)
  (set `self.Hit Sound` _hitsound)
  (set `self.HitSoundThreshold` _hitsoundthreshold)
  (set `self.HitSoundMinVolume` _hitsoundminvolume)
  (set `self.HitSoundMaxVolume` _hitsoundmaxvolume)
  (set `self.Attenuation` _hitsoundattenuation))

(fn `UserConstructionScript`
  (`self.SetupSettings` (`self.Object Mesh`) (`self.Physics Object Settings`) (`self.CreateGameEvents`))
  (`PrimitiveComponent.SetSimulatePhysics` (`self.ObjectMesh`) (`self.SimulatePhysics`))
  (`PrimitiveComponent.SetMassOverrideInKg` (`self.ObjectMesh`) "None" (`self.Mass`) true)
  (`PrimitiveComponent.SetLinearDamping` (`self.ObjectMesh`) (`self.LinearDamping`))
  (`PrimitiveComponent.SetAngularDamping` (`self.ObjectMesh`) (`self.AngularDamping`))
  (`PrimitiveComponent.SetEnableGravity` (`self.ObjectMesh`) (`self.EnableGravity`))
  (`PrimitiveComponent.SetCollisionResponseToChannel` (`self.ObjectMesh`) "ECC_Pawn" "ECR_Block"))