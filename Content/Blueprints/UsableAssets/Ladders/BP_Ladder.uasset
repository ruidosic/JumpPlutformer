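; Usable first-person ladder actor, procedurally built in the construction script from instanced bottom, middle, connect and top meshes, which also positions its interaction points.
; Use toggles holding on: a timeline eases player and camera into place, then Flying movement climbs on forward input, with footstep sounds, optional headshake and optional yaw limits.
; Climbing down past the release height drops the player; reaching the top trigger runs a timeline to the optional final location.
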(event `self.Use`
  (params (GameEvent :type Boolean))
  ;[1 1 1] Interaction Settings
  (`/Game/Blueprints/Core/BPM_CoreEngine.GE_CheckInteraction`)
  (if GameEvent
    _
    (elif (`self.OnLadder`)
      (`self.LeaveLadder`)
      (else
        (bind _as_core_engine (`/Game/Blueprints/Core/BP_Functions.GetPlayer`))
        (bind _currentladder (`/Game/Blueprints/Core/BP_CoreEngine.CurrentLadder` _as_core_engine))
        (`/Engine/EditorBlueprintResources/StandardMacros.IsValid` _currentladder
          (:`Is Valid`
            (`self.LeaveLadder` _currentladder))
          (:`Is Not Valid`
            _))
        (`self.HoldLadder`)))))

(event `InputAxis|MoveForward`
  (params (AxisValue :type "Float (single-precision)"))
  (bind _returnvalue (`GameplayStatics.GetPlayerCharacter` 0))
  (bind (_returnvalue_x _returnvalue_y _returnvalue_z) (`KismetMathLibrary.BreakVector` (`SceneComponent.K2_GetComponentLocation` (`self.ReleaseHeight`))))
  (bind (_returnvalue_x_2 _returnvalue_y_2 _returnvalue_z_2) (`KismetMathLibrary.BreakVector` (`SceneComponent.K2_GetComponentLocation` (`Character.CapsuleComponent` (`GameplayStatics.GetPlayerCharacter` 0)))))
  ;[1 1 1] Interaction Settings
  (if (not (`self.UseTrigger`))
    (`Pawn.AddMovementInput` _returnvalue (`self.GetActorUpVector` _returnvalue) AxisValue false)
    (`self.LadderFootsteps`)
    ;;[1 1 1] Move Bottom and leave
    (if (and (< _returnvalue_z_2 _returnvalue_z) (< AxisValue 0.0))
      (`self.LeaveLadder`))))

(event `InputAxis|LookUp`
  (params (AxisValue :type "Float (single-precision)"))
  ;[1 1 1] Interaction Settings
  (`Pawn.AddControllerPitchInput` (`GameplayStatics.GetPlayerPawn` 0) AxisValue))

(event `InputAxis|LookUpRate`
  (params (AxisValue :type "Float (single-precision)"))
  ;[1 1 1] Interaction Settings
  (bind _as_core_engine (`/Game/Blueprints/Core/BP_Functions.GetPlayer`))
  (`Pawn.AddControllerPitchInput` (`GameplayStatics.GetPlayerPawn` 0) (* AxisValue (`/Game/Blueprints/Core/BP_CoreEngine.BaseLookUpRate` _as_core_engine) (`GameplayStatics.GetWorldDeltaSeconds`))))

(event `self.TopCollision.OnComponentBeginOverlap`
  (params (OverlappedComponent :type "PrimitiveComponent Object Reference") (OtherActor :type "Actor Object Reference") (OtherComp :type "PrimitiveComponent Object Reference") (OtherBodyIndex :type Integer) (bFromSweep :type Boolean) (SweepResult :type "HitResult Structure (by ref)"))
  ;[1 1 1] Interaction Settings
  (if (and (`self.HasFinalLocation`) (== OtherActor (`GameplayStatics.GetPlayerPawn` 0)) (`self.OnLadder`))
    (`self.LeaveLadderTop`)))

(event `InputAxis|Turn`
  (params (AxisValue :type "Float (single-precision)"))
  ;[1 1 1] Interaction Settings
  (`Pawn.AddControllerYawInput` (`GameplayStatics.GetPlayerPawn` 0) AxisValue))

(event `InputAxis|TurnRate`
  (params (AxisValue :type "Float (single-precision)"))
  ;[1 1 1] Interaction Settings
  (bind _as_core_engine (`/Game/Blueprints/Core/BP_Functions.GetPlayer`))
  (`Pawn.AddControllerYawInput` (`GameplayStatics.GetPlayerPawn` 0) (* (`/Game/Blueprints/Core/BP_CoreEngine.BaseTurnRate` _as_core_engine) AxisValue (`GameplayStatics.GetWorldDeltaSeconds`))))

(event `HoldLadder`
  (bind _returnvalue (`GameplayStatics.GetPlayerCameraManager` 0))
  (bind (_startlocation_x _startlocation_y _startlocation_z) (`KismetMathLibrary.BreakVector` (`self.StartLocation`)))
  (bind (_returnvalue_x _returnvalue_y _returnvalue_z) (`KismetMathLibrary.BreakVector` (`SceneComponent.K2_GetComponentLocation` (`self.StartPositionUp`))))
  (bind (_returnvalue_x_2 _returnvalue_y_2 _returnvalue_z_2) (`KismetMathLibrary.BreakVector` (`SceneComponent.K2_GetComponentLocation` (`self.StartPositionDown`))))
  (bind (_returnvalue_roll _returnvalue_pitch _returnvalue_yaw) (`KismetMathLibrary.BreakRotator` (`SceneComponent.K2_GetComponentRotation` (`self.Billboard`))))
  (bind _charactermovement (`Character.CharacterMovement` (`GameplayStatics.GetPlayerCharacter` 0)))
  (bind _updatedprimitive (`MovementComponent.UpdatedPrimitive` (`Character.CharacterMovement` (`GameplayStatics.GetPlayerCharacter` 0))))
  (bind (_returnvalue_x_3 _returnvalue_y_3 _returnvalue_z_3) (`KismetMathLibrary.BreakVector` (`SceneComponent.K2_GetComponentLocation` _updatedprimitive)))
  ;[1 1 1] Hold / Leave Settings
  (if (not (`self.OnLadder`))
    (bind _as_core_engine (`/Game/Blueprints/Core/BP_Functions.GetPlayer`))
    (`/Game/Blueprints/Core/BP_CoreEngine.UnequipAll` _as_core_engine)
    (set `/Game/Blueprints/Core/BP_CoreEngine.OnLadder` true _as_core_engine)
    (set `/Game/Blueprints/Core/BP_CoreEngine.CurrentLadder` self _as_core_engine)
    (set `CharacterMovementComponent.MaxFlySpeed` (`self.ClimbSpeed`) _charactermovement)
    (set `CharacterMovementComponent.BrakingDecelerationFlying` 1000.0 _charactermovement)
    (`CharacterMovementComponent.SetMovementMode` _charactermovement "MOVE_None" 0)
    (set `self.StartLocation` (`SceneComponent.K2_GetComponentLocation` (`MovementComponent.UpdatedPrimitive` _charactermovement)))
    (set `self.StartRotation` (`SceneComponent.K2_GetComponentRotation` (`/Game/Blueprints/Core/BP_CoreEngine.PlayerCamera` _as_core_engine)))
    (`self.ControllerInput` false)
    (`PrimitiveComponent.SetCollisionEnabled` (`Character.CapsuleComponent` (`GameplayStatics.GetPlayerCharacter` 0)) "NoCollision")
    (bind _as_core_engine_2 (`/Game/Blueprints/Core/BP_Functions.GetPlayer`))
    (bind (_direction _animation) (`Timeline|LadderStartTimeline` :!via `PlayFromStart`)
      (:`Update`
        (set `self.InteractionEnabled` false)
        (`SceneComponent.K2_SetWorldLocation` _updatedprimitive (`KismetMathLibrary.VLerp` (`self.StartLocation`) (`KismetMathLibrary.MakeVector` _returnvalue_x _returnvalue_y (select `bool` (or (== (`/Game/Blueprints/Core/BP_CoreEngine.HitComponent` _as_core_engine_2) (`self.LadderTop`)) (<= (.z (`SceneComponent.K2_GetComponentLocation` (`self.StartPositionUp`))) _startlocation_z)) :`false` (select `bool` (> _returnvalue_z_2 (.z (`self.StartLocation`))) :`false` _returnvalue_z_3 :`true` _returnvalue_z_2) :`true` _returnvalue_z)) _animation) true true)
        (`Controller.SetControlRotation` (`GameplayStatics.GetPlayerController` 0) (`KismetMathLibrary.RLerp` (`self.StartRotation`) (`SceneComponent.K2_GetComponentRotation` (`self.StartPositionDown`)) _animation true)))
      (:`Finished`
        (set `self.OnLadder` true)
        (`self.ControllerInput` true)
        (`CharacterMovementComponent.SetMovementMode` (`Character.CharacterMovement` (`GameplayStatics.GetPlayerCharacter` 0)) "MOVE_Flying" 0)
        (if (not (`self.360 View`))
          (set `PlayerCameraManager.ViewYawMin` (+ _returnvalue_yaw 180.0) _returnvalue)
          (set `PlayerCameraManager.ViewYawMax` _returnvalue_yaw _returnvalue))
        (`self.FinalLocationCollision`) ; TopCollision Block Move Up or Overlap Player for event
        (set `self.InteractionEnabled` true)
        (`PrimitiveComponent.SetCollisionEnabled` (`Character.CapsuleComponent` (`GameplayStatics.GetPlayerCharacter` 0)) "QueryAndPhysics")
        (`self.GameEventCheck` "NewEnumerator12")))))

(event `LeaveLadderTop`
  (bind _returnvalue (`GameplayStatics.GetPlayerCameraManager` 0))
  (bind _charactermovement (`Character.CharacterMovement` (`GameplayStatics.GetPlayerCharacter` 0)))
  ;[1 1 1] Hold / Leave Settings
  (if (`self.OnLadder`)
    (bind _as_core_engine (`/Game/Blueprints/Core/BP_Functions.GetPlayer`))
    (`CharacterMovementComponent.SetMovementMode` _charactermovement "MOVE_None" 0)
    (set `self.EndLocation` (`SceneComponent.K2_GetComponentLocation` (`MovementComponent.UpdatedPrimitive` _charactermovement)))
    (set `self.EndRotation` (`SceneComponent.K2_GetComponentRotation` (`/Game/Blueprints/Core/BP_CoreEngine.PlayerCamera` _as_core_engine)))
    (`self.ControllerInput` false)
    (`PrimitiveComponent.SetCollisionEnabled` (`Character.CapsuleComponent` (`GameplayStatics.GetPlayerCharacter` 0)) "NoCollision")
    (bind (_direction _animation) (`Timeline|LadderEndTimeline` :!via `PlayFromStart`)
      (:`Update`
        (set `self.InteractionEnabled` false)
        (`SceneComponent.K2_SetWorldLocation` (`MovementComponent.UpdatedPrimitive` (`Character.CharacterMovement` (`GameplayStatics.GetPlayerCharacter` 0))) (`KismetMathLibrary.VLerp` (`self.EndLocation`) (`SceneComponent.K2_GetComponentLocation` (`self.EndPosition`)) _animation) true true)
        (`Controller.SetControlRotation` (`GameplayStatics.GetPlayerController` 0) (`KismetMathLibrary.RLerp` (`self.EndRotation`) (`SceneComponent.K2_GetComponentRotation` (`self.EndPosition`)) _animation true))
        (`CharacterMovementComponent.SetMovementMode` (`Character.CharacterMovement` (`GameplayStatics.GetPlayerCharacter` 0)) "MOVE_Walking" 0)
        (set `PlayerCameraManager.ViewYawMin` 0.0 _returnvalue)
        (set `PlayerCameraManager.ViewYawMax` 359.899994 _returnvalue))
      (:`Finished`
        (set `self.OnLadder` false)
        (bind _as_core_engine_2 (`/Game/Blueprints/Core/BP_Functions.GetPlayer`))
        (set `/Game/Blueprints/Core/BP_CoreEngine.OnLadder` false _as_core_engine_2)
        (set `/Game/Blueprints/Core/BP_CoreEngine.CurrentLadder` self _as_core_engine_2)
        (set `self.InteractionEnabled` true)
        (`PrimitiveComponent.SetCollisionEnabled` (`Character.CapsuleComponent` (`GameplayStatics.GetPlayerCharacter` 0)) "QueryAndPhysics")
        (`self.GameEventCheck` "NewEnumerator14")))))

(event `LeaveLadder`
  (bind _returnvalue (`GameplayStatics.GetPlayerCameraManager` 0))
  ;[1 1 1] Hold / Leave Settings
  (if (`self.OnLadder`)
    (set `self.OnLadder` false)
    (bind _as_core_engine (`/Game/Blueprints/Core/BP_Functions.GetPlayer`))
    (set `/Game/Blueprints/Core/BP_CoreEngine.OnLadder` false _as_core_engine)
    (`CharacterMovementComponent.SetMovementMode` (`Character.CharacterMovement` (`GameplayStatics.GetPlayerCharacter` 0)) "MOVE_Walking" 0)
    (set `PlayerCameraManager.ViewYawMin` 0.0 _returnvalue)
    (set `PlayerCameraManager.ViewYawMax` 359.899994 _returnvalue)
    (`PrimitiveComponent.SetCollisionResponseToChannel` (`self.TopCollision`) "ECC_Pawn" "ECR_Overlap")
    (bind _as_core_engine_2 (`/Game/Blueprints/Core/BP_Functions.GetPlayer`))
    (set `/Game/Blueprints/Core/BP_CoreEngine.CurrentLadder` self _as_core_engine_2)
    (`self.ControllerInput` false)
    (`self.GameEventCheck` "NewEnumerator13")
    (set `self.InteractionEnabled` false)
    (`KismetSystemLibrary.Delay` 0.5)
    (set `self.InteractionEnabled` true)))

(fn `LadderFootsteps`
  (bind _climbsound (`self.ClimbSound`))
  (bind _capsulecomponent (`Character.CapsuleComponent` (`GameplayStatics.GetPlayerCharacter` 0)))
  (bind _z (.z (`SceneComponent.K2_GetComponentLocation` _capsulecomponent)))
  (if (or (<= (+ (`self.LastFootstepLocation`) (`self.ClimbSoundRate`)) _z) (>= (- (`self.LastFootstepLocation`) (`self.ClimbSoundRate`)) _z))
    (`/Game/Blueprints/Core/BPM_CoreEngine.GE_3DSound` _climbsound false _climbsound _capsulecomponent (`self.Attenuation`))
    (set `self.LastFootstepLocation` _z)
    (if (`self.Headshake`)
      (`PlayerController.ClientStartCameraShake` :`self` (`GameplayStatics.GetPlayerController` 0) :`Shake` "/Game/Blueprints/Core/CameraShakes/HeadShakeLadder.HeadShakeLadder_C" :`Scale` (`self.HeadshakeScale`)))))

(fn `SetupSettings`
  (params (`Trigger Settings` :type "/Game/Blueprints/UsableAssets/Doors/Structs/Struct_TriggerSettings Structure") (`Mesh Settings` :type "/Game/Blueprints/UsableAssets/Ladders/Structs/Struct_LadderMeshSettings Structure") (`Ladder Settings` :type "/Game/Blueprints/UsableAssets/Ladders/Structs/Struct_LadderSettings Structure") (`Game Events` :type "Array of /Game/Blueprints/Events/Structs/Struct_GameEvents Structure") (Attenuation :type "SoundAttenuation Object Reference"))
  (bind (_laddertopmesh _laddermiddlemesh _ladderconnectmesh _ladderbottommesh) (break `/Game/Blueprints/UsableAssets/Ladders/Structs/Struct_LadderMeshSettings` `Mesh Settings`))
  (bind (_usetrigger _triggersize) (break `/Game/Blueprints/UsableAssets/Doors/Structs/Struct_TriggerSettings` `Trigger Settings`))
  (bind (_animationinfo _generationinfo _interactionpoints _movementinfo) (break `/Game/Blueprints/UsableAssets/Ladders/Structs/Struct_LadderSettings` `Ladder Settings`))
  (bind (_ladderholddurationsec _ladderleaveholddurationsec) (break `/Game/Blueprints/UsableAssets/Ladders/Structs/Struct_LadderAnimInfo` _animationinfo))
  (bind (_hasfinallocation _ladderstep _ladderheight _connectrate) (break `/Game/Blueprints/UsableAssets/Ladders/Structs/Struct_LadderGenerationInfo` _generationinfo))
  (bind (_finallocation _releaseheight) (break `/Game/Blueprints/UsableAssets/Ladders/Structs/Struct_LadderInteractionPoints` _interactionpoints))
  (bind (_climbspeed _360view _climbsoundrate _climbsound _headshake _headshakescale) (break `/Game/Blueprints/UsableAssets/Ladders/Structs/Struct_LadderMovementInfo` _movementinfo))
  ;[1 1 1] Setup Use Trigger Configuration
  (set `self.UseTrigger` _usetrigger)
  (set `self.TriggerSize` _triggersize)
  ;[1 1 1] Setup Attenuation Settings
  (set `self.Attenuation` Attenuation)
  ;[1 1 1] Setup Game Events
  (set `self.GameEvents` `Game Events`)
  ;[1 1 1] Setup Meshes Settings
  (set `self.LadderTopMesh` _laddertopmesh)
  (set `self.LadderMiddleMesh` _laddermiddlemesh)
  (set `self.LadderConnectMesh` _ladderconnectmesh)
  (set `self.LadderBottomMesh` _ladderbottommesh)
  ;[1 1 1] Setup Ladder Anim Info
  (set `self.Ladder Hold Duration(Sec)` _ladderholddurationsec)
  (set `self.Ladder Leave Hold Duration(Sec)` _ladderleaveholddurationsec)
  ;[1 1 1] Setup Ladder Generation Info
  (set `self.HasFinalLocation` _hasfinallocation)
  (set `self.LadderStep` _ladderstep)
  (set `self.LadderHeight` _ladderheight)
  (set `self.ConnectRate` _connectrate)
  ;[1 1 1] Setup Ladder Interaction Points
  (set `self.FinalLocation` _finallocation)
  (set `self.Release Height` _releaseheight)
  ;[1 1 1] Setup Ladder Movement Info
  (set `self.ClimbSpeed` _climbspeed)
  (set `self.360 View` _360view)
  (set `self.ClimbSoundRate` _climbsoundrate)
  (set `self.ClimbSound` _climbsound)
  (set `self.Headshake` _headshake)
  (set `self.HeadshakeScale` _headshakescale))

(fn `UserConstructionScript`
  (bind (_finallocation_x _finallocation_y _finallocation_z) (`KismetMathLibrary.BreakVector` (`self.FinalLocation`)))
  (bind _returnvalue (- (`self.LadderStep`) 1))
  (`/Game/Blueprints/Core/BP_Functions.SetMesh` (`self.LadderTop`) (`self.LadderTopMesh`))
  (`/Game/Blueprints/Core/BP_Functions.SetMesh` (`self.LadderMiddle`) (`self.LadderMiddleMesh`))
  (`/Game/Blueprints/Core/BP_Functions.SetMesh` (`self.LadderConnect`) (`self.LadderConnectMesh`))
  (`/Game/Blueprints/Core/BP_Functions.SetMesh` (`self.LadderBottom`) (`self.LadderBottomMesh`))
  (`/Game/Blueprints/Core/BP_Functions.PlayRate` (`self.LadderStartTimeline`) (`self.Ladder Hold Duration(Sec)`))
  (`/Game/Blueprints/Core/BP_Functions.PlayRate` (`self.LadderEndTimeline`) (`self.Ladder Leave Hold Duration(Sec)`))
  (for _index (range (+ _returnvalue 1))
    (if (== _index 0)
      (bind _returnvalue_2 (`KismetMathLibrary.MakeVector` 0.0 0.0 (* _index (`self.LadderHeight`))))
      (`InstancedStaticMeshComponent.AddInstance` (`self.LadderBottom`) (`KismetMathLibrary.MakeTransform` _returnvalue_2))
      (elif (== _index _returnvalue)
        (`InstancedStaticMeshComponent.AddInstance` (`self.LadderTop`) (`KismetMathLibrary.MakeTransform` _returnvalue_2))
        (elif (== (mod _index (`self.ConnectRate`)) 0)
          (`InstancedStaticMeshComponent.AddInstance` (`self.LadderConnect`) (`KismetMathLibrary.MakeTransform` _returnvalue_2))
          (else
            (`InstancedStaticMeshComponent.AddInstance` (`self.LadderMiddle`) (`KismetMathLibrary.MakeTransform` _returnvalue_2)))))))
  (bind _z (.z _returnvalue_2))
  (`SceneComponent.K2_SetRelativeLocation` (`self.EndPosition`) (`KismetMathLibrary.MakeVector` _finallocation_x _finallocation_y (+ _finallocation_z _z)) false false)
  (`SceneComponent.K2_SetRelativeLocationAndRotation` :`self` (`self.StartPositionUp`) :`NewLocation` (`KismetMathLibrary.MakeVector` 0.0 75.0 _z))
  (`SceneComponent.K2_SetRelativeLocation` (`self.TopCollision`) (`KismetMathLibrary.MakeVector` 0.0 40.0 (+ _z 150.0)) false false)
  (`SceneComponent.K2_SetRelativeLocation` (`self.Interaction`) (`KismetMathLibrary.MakeVector` 0.0 10.0 (- (* (`self.LadderStep`) 20.0) 15.0)) false false)
  (`BoxComponent.SetBoxExtent` (`self.Interaction`) (`KismetMathLibrary.MakeVector` 38.0 8.0 (+ (* (`self.LadderStep`) 20.0) 5.0)) true)
  (`SceneComponent.K2_SetRelativeLocation` (`self.ReleaseHeight`) (`KismetMathLibrary.MakeVector` 0.0 30.0 (`self.Release Height`)) false false))