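; BP_KeycardControl is a usable keycard reader that opens and closes its connected doors.
; Use either toggles directly or, with AskForKey, opens the inventory filtered to keycards, with game events bypassing selection.
; Opening requires a held key plus a disarmed state or admin key, otherwise showing a notice or denied feedback.
; Construction adds instanced reader meshes, optionally cloned, and syncs door states; runtime changes swap meshes, play sounds and check game events.
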(event `self.Use`
  (params (GameEvent :type Boolean))
  ;[1 1 1] Use / Alternative Use Events
  (`/Game/Blueprints/Core/BPM_CoreEngine.GE_CheckInteraction` :!label _label)
  (if (`self.AskForKey`)
    (if (or GameEvent (stale `self.AlternativeUse` GameEvent))
      (if (`self.Open`) :!label _label_2
        (`self.Close/Off` false)
        (else
          (`self.Open/On` false)))
      (else
        (`self.SelectKey`)))
    (else
      (goto _label_2))))

(event `self.AlternativeUse`
  (params (GameEvent :type Boolean))
  ;[1 1 1] Use / Alternative Use Events
  (goto _label))

(event `self.Open/On`
  (params (GameEvent :type Boolean))
  ;[1 1 1] Open/On & Close/Off Events
  (`/Game/Blueprints/Core/BPM_CoreEngine.GE_CheckInteraction`)
  (if (`self.PlayerHasKey`)
    (if (`self.Disalarmed`)
      (if (not (`self.Open`)) :!label _label_3
        (set `self.Open` true)
        (`self.Open/On` (`self.ConnectedDoors`) false)
        (`|ExecutionSequence`
          (:`then_0`
            (set `self.InteractionEnabled` false :!label _label_4)
            (`/Game/Blueprints/Core/BP_Functions.SetMesh` (`self.KeycardControl`) (select `bool` (`self.Open`) :`false` (`self.CloseMesh`) :`true` (`self.OpenMesh`)))
            (bind (_sound _duration) (`/Game/Blueprints/Core/BPM_CoreEngine.GE_3DSound` null true (select `bool` (`self.Open`) :`false` (`self.OpenSound`) :`true` (`self.CloseSound`)) (`self.KeycardControl`) (`self.Attenuation`)))
            (`/Engine/EditorBlueprintResources/StandardMacros.IsValid` _sound
              (:`Is Valid`
                (`KismetSystemLibrary.Delay` _duration))
              (:`Is Not Valid`
                _))
            (set `self.InteractionEnabled` true)
            (`self.GameEventCheck` (select `bool` (`self.Open`) :`false` "NewEnumerator2" :`true` "NewEnumerator1" :!type "/Game/Blueprints/Events/Enums/Enum_GameEventCheck Enum")))
          (:`then_1`
            (bind _as_core_engine (`/Game/Blueprints/Core/BP_Functions.GetPlayer`))
            (bind _filteredarray (`KismetArrayLibrary.FilterArray` (`/Game/Blueprints/Core/BP_CoreEngine.PlayerInventory` _as_core_engine) "/Game/Blueprints/UsableAssets/Inventory/Keys/BP_Keycard.BP_Keycard_C"))
            (for _array_element _filteredarray
              (bind _asbp_keycard (cast `/Game/Blueprints/UsableAssets/Inventory/Keys/BP_Keycard` _array_element))
              (`/Game/Blueprints/UsableAssets/Inventory/Keys/BP_Key.CheckUnlocked` _asbp_keycard)))))
      (elif (`self.AdminKey`)
        (goto _label_3)
        (else
          (`self.Denied`))))
    (else
      (`/Game/Blueprints/Core/BP_Functions.Notice` "Need" "Keycard" "to access."))))

(event `self.Close/Off`
  (params (GameEvent :type Boolean))
  ;[1 1 1] Open/On & Close/Off Events
  (`/Game/Blueprints/Core/BPM_CoreEngine.GE_CheckInteraction`)
  (if GameEvent
    (if (`self.Open`) :!label _label_5
      (set `self.Open` false)
      (`self.Close/Off` (`self.ConnectedDoors`) false)
      (goto _label_4))
    (elif (`self.PlayerHasKey`)
      (goto _label_5))))

(event `Denied`
  ;[1 1 1] Denied
  (set `self.InteractionEnabled` false)
  (`/Game/Blueprints/Core/BP_Functions.SetMesh` (`self.KeycardControl`) (`self.DeniedMesh`))
  (bind (_sound _duration) (`/Game/Blueprints/Core/BPM_CoreEngine.GE_3DSound` null true (`self.DeniedSound`) (`self.KeycardControl`) (`self.Attenuation`)))
  (`KismetSystemLibrary.Delay` _duration)
  (`/Game/Blueprints/Core/BP_Functions.SetMesh` (`self.KeycardControl`) (`self.CloseMesh`))
  (set `self.InteractionEnabled` true)
  (`self.GameEventCheck` "NewEnumerator18"))

(event `TakeAdminKey`
  ;[0 0 0] Key Events
  ;;[1 1 1] Take Key / Admin Key
  (set `self.AdminKey` true))

(event `self.TakeKey`
  (params (GameEvent :type Boolean))
  ;[0 0 0] Key Events
  ;;[1 1 1] Take Key / Admin Key
  (set `self.PlayerHasKey` true))

(event `SelectKey`
  ;[0 0 0] Key Events
  ;;[1 1 1] Select Key
  (bind _as_core_engine (`/Game/Blueprints/Core/BP_Functions.GetPlayer`))
  (if (`/Game/Blueprints/Core/BP_CoreEngine.FilterInventory` _as_core_engine)
    (bind _filteredarray (`KismetArrayLibrary.FilterArray` (`/Game/Blueprints/Core/BP_CoreEngine.PlayerInventory` _as_core_engine) "/Game/Blueprints/UsableAssets/Inventory/Keys/BP_Keycard.BP_Keycard_C"))
    (if (> (`KismetArrayLibrary.Array_Length` _filteredarray) 0)
      (set `/Game/Blueprints/Core/BP_CoreEngine.InventoryFilter` "NewEnumerator3" _as_core_engine)
      (set `/Game/Blueprints/Core/BP_CoreEngine.UsableRef` self _as_core_engine)
      (`/Game/Blueprints/Core/BP_Functions.SetFilteredItems` "/Game/Blueprints/UsableAssets/Inventory/Keys/BP_Keycard.BP_Keycard_C" true true (select `bool` (`self.Open`) :`false` "Access" :`true` "Lock" :!type "Text"))
      (`/Game/Blueprints/Core/BP_Functions.OpenInventory`)
      (else
        (`/Game/Blueprints/Core/BP_Functions.Notice` "There is no any" "Keycard" "in inventory.")))))

(fn `UserConstructionScript`
  (`parent.UserConstructionScript`)
  (if (`self.CloneMesh`)
    (`InstancedStaticMeshComponent.AddInstance` (`self.KeycardControl`) (`KismetMathLibrary.MakeTransform` (`self.CloneMeshLocation`) (`self.CloneMeshRotation`))))
  (`InstancedStaticMeshComponent.AddInstance` (`self.KeycardControl`) (`KismetMathLibrary.MakeTransform` (0.0 0.0 0.0)))
  (`/Game/Blueprints/Core/BP_Functions.SetMesh` (`self.KeycardControl`) (select `bool` (`self.Open`) :`false` (`self.OpenMesh`) :`true` (`self.CloseMesh`)))
  ;[1 1 1] Change Doors State Depends by Open : Open/Close Location, Timeline On/Off Time
  (for _array_element (`self.ConnectedDoors`)
    (set `/Game/Blueprints/UsableAssets/Doors/BP_Door.Open` (`self.Open`) _array_element)
    (`/Game/Blueprints/UsableAssets/Doors/BP_ControlledDoor.RefreshDoor` _array_element)))