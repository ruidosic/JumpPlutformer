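; Usable monitor that shows render-target feeds from connected security-style cameras and can be switched on or off.
; Use toggles power, while AlternativeUse cycles through ConnectedCameras with wraparound when powered; both report game events.
; RefreshScreen feeds the selected camera's render target, or black when off, into a dynamic screen material, swapping materials if that camera is off.
; The construction script applies mesh and materials, then refreshes the screen.
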(event `self.ReceiveBeginPlay`
  (`self.RefreshScreen`))

(event `self.Open/On`
  (params (GameEvent :type Boolean))
  ;[1 1 1] On / Close Events
  (`/Game/Blueprints/Core/BPM_CoreEngine.GE_CheckInteraction`)
  (set `self.On / Off` true)
  (`self.RefreshScreen` :!label _label)
  (`self.GameEventCheck` (select `bool` (`self.On / Off`) :`false` "NewEnumerator1" :`true` "NewEnumerator2" :!type "/Game/Blueprints/Events/Enums/Enum_GameEventCheck Enum")))

(event `self.Use`
  (params (GameEvent :type Boolean))
  ;[1 1 1] Use Events
  (`/Game/Blueprints/Core/BPM_CoreEngine.GE_CheckInteraction`)
  (if (`self.On / Off`)
    (`self.Close/Off` false)
    (else
      (`self.Open/On` false))))

(event `self.Close/Off`
  (params (GameEvent :type Boolean))
  ;[1 1 1] On / Close Events
  (`/Game/Blueprints/Core/BPM_CoreEngine.GE_CheckInteraction`)
  (set `self.On / Off` false)
  (goto _label))

(event `self.AlternativeUse`
  (params (GameEvent :type Boolean))
  ;[1 1 1] Use Events
  (`/Game/Blueprints/Core/BPM_CoreEngine.GE_CheckInteraction`)
  (if (`self.On / Off`)
    (`self.SwitchCamera`)))

(event `SwitchCamera`
  ;[1 1 1] Switch Camera Settings
  (`/Engine/EditorBlueprintResources/StandardMacros.IncrementInt` (`self.StartCamera`)
    (:`  `
      (if (not (`KismetArrayLibrary.Array_IsValidIndex` (`self.ConnectedCameras`) (`self.StartCamera`)))
        (set `self.StartCamera` 0))
      (`self.RefreshScreen`)
      (`self.GameEventCheck` "NewEnumerator33"))))

(fn `RefreshScreen`
  (if (`self.On / Off`)
    (`MaterialInstanceDynamic.SetTextureParameterValue` (`self.ScreenMaterialRef`) "Texture" (select `bool` (`self.On / Off`) :`false` "/Game/Assets/MeshMat/Monitor/RT_EmptyBlack.RT_EmptyBlack" :`true` (`/Game/Blueprints/UsableAssets/Electronics/BP_Camera.RenderTarget` (`|GetArrayItem` (`self.ConnectedCameras`) (`self.StartCamera`))) :!type "Texture Object Reference"))
    (`PrimitiveComponent.SetMaterial` (`self.Monitor`) 1 (select `bool` (`/Game/Blueprints/UsableAssets/Electronics/BP_Camera.On / Off` (`|GetArrayItem` (`self.ConnectedCameras`) (`self.StartCamera`))) :`true` (`self.ScreenMaterialRef`) :!type "MaterialInterface Object Reference"))
    (set `self.StartCamera` (`KismetMathLibrary.Clamp` (`self.StartCamera`) 0 (`KismetArrayLibrary.Array_LastIndex` (`self.ConnectedCameras`))))
    (else
      (`MaterialInstanceDynamic.SetTextureParameterValue` (`self.ScreenMaterialRef`) "Texture" "/Game/Assets/MeshMat/Monitor/RT_EmptyBlack.RT_EmptyBlack")
      (`PrimitiveComponent.SetMaterial` (`self.Monitor`) 1 (`self.ScreenMaterialRef`)))))

(fn `UserConstructionScript`
  (`parent.UserConstructionScript`)
  (`StaticMeshComponent.SetStaticMesh` (`self.Monitor`) (`self.MonitorMesh`))
  (`PrimitiveComponent.SetMaterial` (`self.Monitor`) 0 (`self.MonitorMaterial`))
  (bind _returnvalue (`PrimitiveComponent.CreateDynamicMaterialInstance` (`self.Monitor`) 0 (`self.ScreenMaterial`) "None"))
  (set `self.ScreenMaterialRef` _returnvalue)
  (`self.RefreshScreen`))