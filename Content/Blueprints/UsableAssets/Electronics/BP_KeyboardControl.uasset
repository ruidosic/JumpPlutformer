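; Usable keypad control panel that locks and unlocks a security system of linked cameras and alarms with a four-digit code.
; Button presses read digits from component tags, driving screen material, button animation and 3D sounds.
; Player detection starts a warning countdown; expiry or repeated wrong codes can trigger alarms and shut off linked keycard controls.
; The correct code unlocks and disarms, repeated Reset presses relock, and key transitions report game events.
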(event `WrongScreen`
  ;[1 1 1] Digit Screen
  (`|ExecutionSequence`
    (:`then_0`
      (`KismetSystemLibrary.Delay` 0.2)
      (set `self.InteractionEnabled` false)
      (`KismetSystemLibrary.Delay` 0.8)
      (set `self.InteractionEnabled` true)
      (set `self.CurrentScreen` null))
    (:`then_1`
      (set `self.CurrentScreenEmissive` 100.0)
      (set `self.CurrentScreen` null)))
  (bind _returnvalue (`PrimitiveComponent.CreateDynamicMaterialInstance` (`self.ControlPanelMesh`) 1 "/Game/HorrorEngine/Materials/HE_ControlScreen.HE_ControlScreen" "None" :!label _label))
  (`MaterialInstanceDynamic.SetTextureParameterValue` _returnvalue "Texture" (`self.CurrentScreen`))
  (`MaterialInstanceDynamic.SetScalarParameterValue` _returnvalue "Emissive" (`self.CurrentScreenEmissive`)))

(event `ButtonSound`
  (bind _returnvalue (select `bool` (`self.Empty Button`) :`false` (`self.Button Sound`) :`true` (`self.Empty Button Sound`)))
  ;[1 1 1] Sound Settings
  (`/Game/Blueprints/Core/BPM_CoreEngine.GE_3DSound` _returnvalue false _returnvalue (`self.ControlPanelMesh`) (`self.Attenuation`)))

(event `CorrectScreen`
  ;[1 1 1] Digit Screen
  (set `self.CurrentScreenEmissive` 20.0)
  (set `self.CurrentScreen` null)
  (goto _label))

(event `WrongCodeSound`
  (bind _wrong_code_sound (`self.Wrong Code Sound`))
  ;[1 1 1] Sound Settings
  (`/Game/Blueprints/Core/BPM_CoreEngine.GE_3DSound` _wrong_code_sound false _wrong_code_sound (`self.ControlPanelMesh`) (`self.Attenuation`)))

(event `DigitScreen`
  ;[1 1 1] Digit Screen
  (set `self.CurrentScreenEmissive` 20.0)
  (set `self.CurrentScreen` (select `int` (`KismetArrayLibrary.Array_Length` (`self.CurrentValues`)) :`0` null :`1` null :`2` null :`3` null :!type "Texture2D Object Reference"))
  (goto _label))

(event `CorrectCodeSound`
  (bind _correct_code_sound (`self.Correct Code Sound`))
  ;[1 1 1] Sound Settings
  (`/Game/Blueprints/Core/BPM_CoreEngine.GE_3DSound` _correct_code_sound false _correct_code_sound (`self.ControlPanelMesh`) (`self.Attenuation`)))

(event `WarningSound`
  (bind _warning_sound (`self.Warning Sound`))
  ;[1 1 1] Sound Settings
  (`/Game/Blueprints/Core/BPM_CoreEngine.GE_3DSound` _warning_sound false _warning_sound (`self.ControlPanelMesh`) (`self.Attenuation`)))

(event `self.Alarm`
  (params (GameEvent :type Boolean))
  ;[1 1 1] Alarm / Disalarm
  (if (not (`self.AlarmStarted`))
    (set `self.AlarmStarted` true)
    (if (not (`self.Locked`))
      (`self.Lock` false))
    (`self.AlarmSound`)
    (`self.Alarm` (`self.Connected Alarms`) false)
    (`self.GameEventCheck` "NewEnumerator34")
    (`self.Close/Off` (`self.Connected Keycard Controls`) false)
    (for _array_element (`self.Connected Keycard Controls`)
      (set `/Game/Blueprints/UsableAssets/Electronics/BP_KeycardControl.Disalarmed` false _array_element))))

(event `ButtonAnimation`
  (bind _currentbutton (`self.CurrentButton`))
  ;[1 1 1] Button Animation
  (set `self.InteractionEnabled` false)
  (bind (_direction _animation) (`Timeline|ButtonTimeline` :!via `PlayFromStart`)
    (:`Update`
      (`/Engine/EditorBlueprintResources/StandardMacros.IsValid` _currentbutton
        (:`Is Valid`
          (`SceneComponent.K2_SetRelativeLocation` _currentbutton (`KismetMathLibrary.MakeVector` (.x (`SceneComponent.RelativeLocation` _currentbutton)) (`KismetMathLibrary.Lerp` 2.0 1.7 _animation) (.z (`SceneComponent.RelativeLocation` _currentbutton))) false false))))
    (:`Finished`
      (set `self.InteractionEnabled` true))))

(event `AlarmSound`
  (bind _alarm_sound (`self.Alarm Sound`))
  ;[1 1 1] Sound Settings
  (`/Game/Blueprints/Core/BPM_CoreEngine.GE_3DSound` _alarm_sound false _alarm_sound (`self.ControlPanelMesh`) (`self.Alarm Attenuation`)))

(event `self.Disalarm`
  (params (GameEvent :type Boolean))
  ;[1 1 1] Alarm / Disalarm
  (if (`self.AlarmStarted`)
    (set `self.AlarmStarted` false)
    (`/Game/Blueprints/Core/BPM_CoreEngine.GE_Stop3DSound ` (`self.Alarm Sound`))
    (`self.Disalarm` (`self.Connected Alarms`) false)
    (`self.GameEventCheck` "NewEnumerator35")
    (for _array_element (`self.Connected Keycard Controls`)
      (set `/Game/Blueprints/UsableAssets/Electronics/BP_KeycardControl.Disalarmed` true _array_element))))

(event `PlayerDetected`
  ;[1 1 1] Payer Detected
  (if (`self.Locked`)
    (if (not (`self.AlarmStarted`))
      (`self.GameEventCheck` "NewEnumerator32")
      (`self.WarningSound` :!label _label_2)
      (set `self.Detected` true)
      (bind (_direction _remainingtime) (`Timeline|WarningTimeline` :!label _label_3)
        (:`Update`
          (set `self.WarningTime` _remainingtime))
        (:`Alarm`
          (`/Game/Blueprints/Core/BPM_CoreEngine.GE_Stop3DSound ` (`self.Warning Sound`))
          (`self.Alarm` false)
          (`self.RemoveWarning`))))))

(event `Warning`
  ;[1 1 1] Payer Detected
  (goto _label_2))

(event `self.Lock`
  (params (GameEvent :type Boolean))
  ;[1 1 1] Lock / Unlock Events
  (set `self.CurrentValues` (`self.Reset`))
  (`self.DigitScreen`)
  (`self.WrongCodeSound`)
  (set `self.Locked` true)
  (set `self.Empty Button` false)
  (`self.Open/On` (`self.Connected Cameras`) false)
  (`self.Open/On` (`self.Connected Alarms`) false)
  (`self.GameEventCheck` "NewEnumerator8"))

(event `RemoveWarning`
  ;[1 1 1] Payer Detected
  (set `self.Detected` false)
  (set `self.WarningTime` 0.0)
  (`|ExecutionSequence`
    (:`then_0`
      (goto _label_3 :!via `Stop`))
    (:`then_1`
      (goto _label_3 :!via `SetNewTime`))))

(event `self.Unlock`
  (params (GameEvent :type Boolean))
  ;[1 1 1] Lock / Unlock Events
  (`/Game/Blueprints/Core/BPM_CoreEngine.GE_Stop3DSound ` (`self.Warning Sound`))
  (`self.CorrectScreen`)
  (`self.CorrectCodeSound`)
  (set `self.Locked` false)
  (set `self.Empty Button` true)
  (`self.Close/Off` (`self.Connected Cameras`) false)
  (`self.Close/Off` (`self.Connected Alarms`) false)
  (set `self.AlarmCounter` 0)
  (`self.Disalarm` false)
  (`self.GameEventCheck` "NewEnumerator9"))

(event `self.Use`
  (params (GameEvent :type Boolean))
  (bind _currentvalues (`self.CurrentValues`))
  ;[1 1 1] Use Event
  (`/Game/Blueprints/Core/BPM_CoreEngine.GE_CheckInteraction`)
  (bind _as_core_engine (`/Game/Blueprints/Core/BP_Functions.GetPlayer`))
  (set `self.CurrentButton` (`/Game/Blueprints/Core/BP_CoreEngine.HitComponent` _as_core_engine))
  (`self.ButtonAnimation`)
  (if (`self.Locked`)
    ;;[1 1 1] Press Reset / Enter
    (if (or (== (`self.CurrentButton`) (`self.ButtonEnter`)) (== (`self.CurrentButton`) (`self.ButtonReset`)))
      ;;[1 1 1] Pressed Reset Button?
      (if (== (`self.CurrentButton`) (`self.ButtonReset`))
        ;;[1 1 1] Press Reset
        (set `self.CurrentValues` (`self.Reset`))
        (`self.DigitScreen`)
        (`self.ButtonSound`)
        (set `self.Empty Button` false)
        (else
          ;;[1 1 1] Press Enter
          (if (== (`KismetArrayLibrary.Array_Length` (`self.CurrentValues`)) 4)
            ;;[1 1 1] Entered Code Correct?
            (if (== (+ (* (`|GetArrayItem` _currentvalues) 1000) (* (`|GetArrayItem` _currentvalues 1) 100) (* (`|GetArrayItem` _currentvalues 2) 10) (* (`|GetArrayItem` _currentvalues 3) 1)) (`self.Password`))
              ;;[1 1 1] Unlock
              (`self.Unlock` false)
              (`self.ButtonSound`)
              (`self.RemoveWarning`)
              (else
                ;;[1 1 1] Wrong Code
                (set `self.CurrentValues` (`self.Reset`) :!label _label_4)
                (`self.WrongScreen`)
                (set `self.Empty Button` false)
                (`self.ButtonSound`)
                (`self.WrongCodeSound`)
                (`self.GameEventCheck` "NewEnumerator18")
                ;;[1 1 1] Alarm (if it needed)
                (if (`self.AlarmAfterWrongCode`)
                  (bind _result (`/Engine/EditorBlueprintResources/StandardMacros.IncrementInt` (`self.AlarmCounter`))
                    (:`  `
                      (if (== _result (`self.Alarm After (N) Times Wrong Code`))
                        (`self.Alarm` false)))))))
            (else
              (goto _label_4)))))
      (else
        ;;[1 1 1] Entered 4 Digits?
        (if (>= (`KismetArrayLibrary.Array_Length` (`self.CurrentValues`)) 4)
          ;;[1 1 1] Disable Digital Button Sound
          (set `self.Empty Button` true)
          (`self.ButtonSound`)
          (else
            ;;[1 1 1] Set Digit
            (`KismetArrayLibrary.Array_Add` (`self.CurrentValues`) (`KismetStringLibrary.Conv_StringToInt` (`KismetStringLibrary.Conv_NameToString` (`|GetArrayItem` (`ActorComponent.ComponentTags` (`self.CurrentButton`))))))
            (`self.DigitScreen`)
            (set `self.Empty Button` false)
            (`self.ButtonSound`)))))
    (else
      ;;[1 1 1] Check For Lock
      (`self.ButtonSound`)
      (`|ExecutionSequence`
        (:`then_0`
          (`KismetSystemLibrary.RetriggerableDelay` 3.0)
          (set `self.ResetButtonCounter` 0))
        (:`then_1`
          (if (== (`self.CurrentButton`) (`self.ButtonReset`))
            (bind _result_2 (`/Engine/EditorBlueprintResources/StandardMacros.IncrementInt` (`self.ResetButtonCounter`))
              (:`  `
                (if (== _result_2 (`self.Press Reset (N) Times To Lock`))
                  (`self.Lock` false))))))))))

(fn `UserConstructionScript`
  (`parent.UserConstructionScript`)
  (set `self.GameEvents` (`self.CreateGameEvent`)))