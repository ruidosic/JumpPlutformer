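; Usable climbable ladder that the player can grab, climb and leave, firing game events along the way.
; Construction script stacks instanced mesh segments by step count and positions the start, end, trigger and interaction components to fit.
; Grabbing uses a timeline to lerp player and view into place, then enables Flying movement, optional yaw limits and distance-based climb sounds/shake.
; Descending below release height drops off; the top either blocks or lerps to a final location.
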(event `self.Use`
  (params (GameEvent :type Boolean))
  ;[1 1 1] Interaction Settings
  (`/Game/Blueprints/Core/BPM_CoreEngine.GE_CheckInteraction`)
  (if GameEvent
    _
    (elif (`self.OnLadder`)
      (`self.LeaveLadder`)
      (else
        (bind _as_core_engine (`/Game/Blueprints/Core/BP_Functions.GetPlayer`))
        (bind _currentladder (`/Game/Blueprints/Core/BP_CoreEngine.CurrentLadder` _as_core_engine))
        (`/Engine/EditorBlueprintResources/StandardMacros.IsValid` _currentladder
          (:`Is Valid`
            (`self.LeaveLadder` _currentladder))
          (:`Is Not Valid`
            _))
        (`self.HoldLadder`)))))

(event `InputAxis|MoveForward`
  (params (AxisValue :type "Float (single-precision)"))
  (bind _returnvalue (`GameplayStatics.GetPlayerCharacter` 0))
  (bind (_returnvalue_x _returnvalue_y _returnvalue_z) (`KismetMathLibrary.BreakVector` (`SceneComponent.K2_GetComponentLocation` (`self.ReleaseHeight`))))
  (bind (_returnvalue_x_2 _returnvalue_y_2 _returnvalue_z_2) (`KismetMathLibrary.BreakVector` (`SceneComponent.K2_GetComponentLocation` (`Character.CapsuleComponent` (`GameplayStatics.GetPlayerCharacter` 0)))))
  ;[1 1 1] Interaction Settings
  (if (not (`self.UseTrigger`))
    (`Pawn.AddMovementInput` _returnvalue (`self.GetActorUpVector` _returnvalue) AxisValue false)
    (`self.LadderFootsteps`)
    ;;[1 1 1] Move Bottom and leave
    (if (and (< _returnvalue_z_2 _returnvalue_z) (< AxisValue 0.0))
      (`self.LeaveLadder`))))

(event `InputAxis|LookUp`
  (params (AxisValue :type "Float (single-precision)"))
  ;[1 1 1] Interaction Settings
  (`Pawn.AddControllerPitchInput` (`GameplayStatics.GetPlayerPawn` 0) AxisValue))

(event `InputAxis|LookUpRate`
  (params (AxisValue :type "Float (single-precision)"))
  ;[1 1 1] Interaction Settings
  (bind _as_core_engine (`/Game/Blueprints/Core/BP_Functions.GetPlayer`))
  (`Pawn.AddControllerPitchInput` (`GameplayStatics.GetPlayerPawn` 0) (* AxisValue (`/Game/Blueprints/Core/BP_CoreEngine.BaseLookUpRate` _as_core_engine) (`GameplayStatics.GetWorldDeltaSeconds`))))

(event `self.TopCollision.OnComponentBeginOverlap`
  (params (OverlappedComponent :type "PrimitiveComponent Object Reference") (OtherActor :type "Actor Object Reference") (OtherComp :type "PrimitiveComponent Object Reference") (OtherBodyIndex :type Integer) (bFromSweep :type Boolean) (SweepResult :type "HitResult Structure (by ref)"))
  ;[1 1 1] Interaction Settings
  (if (and (`self.HasFinalLocation`) (== OtherActor (`GameplayStatics.GetPlayerPawn` 0)) (`self.OnLadder`))
    (`self.LeaveLadderTop`)))

(event `InputAxis|Turn`
  (params (AxisValue :type "Float (single-precision)"))
  ;[1 1 1] Interaction Settings
  (`Pawn.AddControllerYawInput` (`GameplayStatics.GetPlayerPawn` 0) AxisValue))

(event `InputAxis|TurnRate`
  (params (AxisValue :type "Float (single-precision)"))
  ;[1 1 1] Interaction Settings
  (bind _as_core_engine (`/Game/Blueprints/Core/BP_Functions.GetPlayer`))
  (`Pawn.AddControllerYawInput` (`GameplayStatics.GetPlayerPawn` 0) (* (`/Game/Blueprints/Core/BP_CoreEngine.BaseTurnRate` _as_core_engine) AxisValue (`GameplayStatics.GetWorldDeltaSeconds`))))

(event `HoldLadder`
  (bind _returnvalue (`GameplayStatics.GetPlayerCameraManager` 0))
  (bind (_startlocation_x _startlocation_y _startlocation_z) (`KismetMathLibrary.BreakVector` (`self.StartLocation`)))
  (bind (_returnvalue_x _returnvalue_y _returnvalue_z) (`KismetMathLibrary.BreakVector` (`SceneComponent.K2_GetComponentLocation` (`self.StartPositionUp`))))
  (bind (_returnvalue_x_2 _returnvalue_y_2 _returnvalue_z_2) (`KismetMathLibrary.BreakVector` (`SceneComponent.K2_GetComponentLocation` (`self.StartPositionDown`))))
  (bind (_returnvalue_roll _returnvalue_pitch _returnvalue_yaw) (`KismetMathLibrary.BreakRotator` (`SceneComponent.K2_GetComponentRotation` (`self.Billboard`))))
  (bind _charactermovement (`Character.CharacterMovement` (`GameplayStatics.GetPlayerCharacter` 0)))
  (bind _updatedprimitive (`MovementComponent.UpdatedPrimitive` (`Character.CharacterMovement` (`GameplayStatics.GetPlayerCharacter` 0))))
  (bind (_returnvalue_x_3 _returnvalue_y_3 _returnvalue_z_3) (`KismetMathLibrary.BreakVector` (`SceneComponent.K2_GetComponentLocation` _updatedprimitive)))
  ;[1 1 1] Hold / Leave Settings
  (if (not (`self.OnLadder`))
    (bind _as_core_engine (`/Game/Blueprints/Core/BP_Functions.GetPlayer`))
    (`/Game/Blueprints/Core/BP_CoreEngine.UnequipAll` _as_core_engine)
    (set `/Game/Blueprints/Core/BP_CoreEngine.OnLadder` true _as_core_engine)
    (set `/Game/Blueprints/Core/BP_CoreEngine.CurrentLadder` self _as_core_engine)
    (set `CharacterMovementComponent.MaxFlySpeed` (`self.ClimbSpeed`) _charactermovement)
    (set `CharacterMovementComponent.BrakingDecelerationFlying` 1000.0 _charactermovement)
    (`CharacterMovementComponent.SetMovementMode` _charactermovement "MOVE_None" 0)
    (set `self.StartLocation` (`SceneComponent.K2_GetComponentLocation` (`MovementComponent.UpdatedPrimitive` _charactermovement)))
    (set `self.StartRotation` (`SceneComponent.K2_GetComponentRotation` (`/Game/Blueprints/Core/BP_CoreEngine.PlayerCamera` _as_core_engine)))
    (`self.ControllerInput` false)
    (`PrimitiveComponent.SetCollisionEnabled` (`Character.CapsuleComponent` (`GameplayStatics.GetPlayerCharacter` 0)) "NoCollision")
    (bind _as_core_engine_2 (`/Game/Blueprints/Core/BP_Functions.GetPlayer`))
    (bind (_direction _animation) (`Timeline|LadderStartTimeline` :!via `PlayFromStart`)
      (:`Update`
        (set `self.InteractionEnabled` false)
        (`SceneComponent.K2_SetWorldLocation` _updatedprimitive (`KismetMathLibrary.VLerp` (`self.StartLocation`) (`KismetMathLibrary.MakeVector` _returnvalue_x _returnvalue_y (select `bool` (or (== (`/Game/Blueprints/Core/BP_CoreEngine.HitComponent` _as_core_engine_2) (`self.LadderTop`)) (<= (.z (`SceneComponent.K2_GetComponentLocation` (`self.StartPositionUp`))) _startlocation_z)) :`false` (select `bool` (> _returnvalue_z_2 (.z (`self.StartLocation`))) :`false` _returnvalue_z_3 :`true` _returnvalue_z_2) :`true` _returnvalue_z)) _animation) true true)
        (`Controller.SetControlRotation` (`GameplayStatics.GetPlayerController` 0) (`KismetMathLibrary.RLerp` (`self.StartRotation`) (`SceneComponent.K2_GetComponentRotation` (`self.StartPositionDown`)) _animation true)))
      (:`Finished`
        (set `self.OnLadder` true)
        (`self.ControllerInput` true)
        (`CharacterMovementComponent.SetMovementMode` (`Character.CharacterMovement` (`GameplayStatics.GetPlayerCharacter` 0)) "MOVE_Flying" 0)
        (if (not (`self.360 View`))
          (set `PlayerCameraManager.ViewYawMin` (+ _returnvalue_yaw 180.0) _returnvalue)
          (set `PlayerCameraManager.ViewYawMax` _returnvalue_yaw _returnvalue))
        (`self.FinalLocationCollision`) ; TopCollision Block Move Up or Overlap Player for event
        (set `self.InteractionEnabled` true)
        (`PrimitiveComponent.SetCollisionEnabled` (`Character.CapsuleComponent` (`GameplayStatics.GetPlayerCharacter` 0)) "QueryAndPhysics")
        (`self.GameEventCheck` "NewEnumerator12")))))

(event `LeaveLadderTop`
  (bind _returnvalue (`GameplayStatics.GetPlayerCameraManager` 0))
  (bind _charactermovement (`Character.CharacterMovement` (`GameplayStatics.GetPlayerCharacter` 0)))
  ;[1 1 1] Hold / Leave Settings
  (if (`self.OnLadder`)
    (bind _as_core_engine (`/Game/Blueprints/Core/BP_Functions.GetPlayer`))
    (`CharacterMovementComponent.SetMovementMode` _charactermovement "MOVE_None" 0)
    (set `self.EndLocation` (`SceneComponent.K2_GetComponentLocation` (`MovementComponent.UpdatedPrimitive` _charactermovement)))
    (set `self.EndRotation` (`SceneComponent.K2_GetComponentRotation` (`/Game/Blueprints/Core/BP_CoreEngine.PlayerCamera` _as_core_engine)))
    (`self.ControllerInput` false)
    (`PrimitiveComponent.SetCollisionEnabled` (`Character.CapsuleComponent` (`GameplayStatics.GetPlayerCharacter` 0)) "NoCollision")
    (bind (_direction _animation) (`Timeline|LadderEndTimeline` :!via `PlayFromStart`)
      (:`Update`
        (set `self.InteractionEnabled` false)
        (`SceneComponent.K2_SetWorldLocation` (`MovementComponent.UpdatedPrimitive` (`Character.CharacterMovement` (`GameplayStatics.GetPlayerCharacter` 0))) (`KismetMathLibrary.VLerp` (`self.EndLocation`) (`SceneComponent.K2_GetComponentLocation` (`self.EndPosition`)) _animation) true true)
        (`Controller.SetControlRotation` (`GameplayStatics.GetPlayerController` 0) (`KismetMathLibrary.RLerp` (`self.EndRotation`) (`SceneComponent.K2_GetComponentRotation` (`self.EndPosition`)) _animation true))
        (`CharacterMovementComponent.SetMovementMode` (`Character.CharacterMovement` (`GameplayStatics.GetPlayerCharacter` 0)) "MOVE_Walking" 0)
        (set `PlayerCameraManager.ViewYawMin` 0.0 _returnvalue)
        (set `PlayerCameraManager.ViewYawMax` 359.899994 _returnvalue))
      (:`Finished`
        (set `self.OnLadder` false)
        (bind _as_core_engine_2 (`/Game/Blueprints/Core/BP_Functions.GetPlayer`))
        (set `/Game/Blueprints/Core/BP_CoreEngine.OnLadder` false _as_core_engine_2)
        (set `/Game/Blueprints/Core/BP_CoreEngine.CurrentLadder` self _as_core_engine_2)
        (set `self.InteractionEnabled` true)
        (`PrimitiveComponent.SetCollisionEnabled` (`Character.CapsuleComponent` (`GameplayStatics.GetPlayerCharacter` 0)) "QueryAndPhysics")
        (`self.GameEventCheck` "NewEnumerator14")))))

(event `LeaveLadder`
  (bind _returnvalue (`GameplayStatics.GetPlayerCameraManager` 0))
  ;[1 1 1] Hold / Leave Settings
  (if (`self.OnLadder`)
    (set `self.OnLadder` false)
    (bind _as_core_engine (`/Game/Blueprints/Core/BP_Functions.GetPlayer`))
    (set `/Game/Blueprints/Core/BP_CoreEngine.OnLadder` false _as_core_engine)
    (`CharacterMovementComponent.SetMovementMode` (`Character.CharacterMovement` (`GameplayStatics.GetPlayerCharacter` 0)) "MOVE_Walking" 0)
    (set `PlayerCameraManager.ViewYawMin` 0.0 _returnvalue)
    (set `PlayerCameraManager.ViewYawMax` 359.899994 _returnvalue)
    (`PrimitiveComponent.SetCollisionResponseToChannel` (`self.TopCollision`) "ECC_Pawn" "ECR_Overlap")
    (bind _as_core_engine_2 (`/Game/Blueprints/Core/BP_Functions.GetPlayer`))
    (set `/Game/Blueprints/Core/BP_CoreEngine.CurrentLadder` self _as_core_engine_2)
    (`self.ControllerInput` false)
    (`self.GameEventCheck` "NewEnumerator13")
    (set `self.InteractionEnabled` false)
    (`KismetSystemLibrary.Delay` 0.5)
    (set `self.InteractionEnabled` true)))

(fn `LadderFootsteps`
  (bind _climbsound (`self.ClimbSound`))
  (bind _capsulecomponent (`Character.CapsuleComponent` (`GameplayStatics.GetPlayerCharacter` 0)))
  (bind _z (.z (`SceneComponent.K2_GetComponentLocation` _capsulecomponent)))
  (if (or (<= (+ (`self.LastFootstepLocation`) (`self.ClimbSoundRate`)) _z) (>= (- (`self.LastFootstepLocation`) (`self.ClimbSoundRate`)) _z))
    (`/Game/Blueprints/Core/BPM_CoreEngine.GE_3DSound` _climbsound false _climbsound _capsulecomponent (`self.SoundAttenuation`))
    (set `self.LastFootstepLocation` _z)
    (if (`self.Headshake`)
      (`PlayerController.ClientStartCameraShake` :`self` (`GameplayStatics.GetPlayerController` 0) :`Shake` "/Game/Blueprints/Core/CameraShakes/HeadShakeLadder.HeadShakeLadder_C" :`Scale` (`self.HeadshakeScale`)))))

(fn `UserConstructionScript`
  (bind (_finallocation_x _finallocation_y _finallocation_z) (`KismetMathLibrary.BreakVector` (`self.FinalLocation`)))
  (bind _returnvalue (- (`self.LadderStep`) 1))
  (`parent.UserConstructionScript`)
  (set `self.GameEvents` (`self.CreateGameEvents`))
  (`/Game/Blueprints/Core/BP_Functions.PlayRate` (`self.LadderStartTimeline`) (`self.StartAnimationDuration(Sec)`))
  (`/Game/Blueprints/Core/BP_Functions.PlayRate` (`self.LadderEndTimeline`) (`self.EndAnimationDuration(Sec)`))
  (for _index (range (+ _returnvalue 1))
    (if (== _index 0)
      (bind _returnvalue_2 (`KismetMathLibrary.MakeVector` 0.0 0.0 (* _index (`self.LadderHeight`))))
      (`InstancedStaticMeshComponent.AddInstance` (`self.LadderBottom`) (`KismetMathLibrary.MakeTransform` _returnvalue_2))
      (elif (== _index _returnvalue)
        (`InstancedStaticMeshComponent.AddInstance` (`self.LadderTop`) (`KismetMathLibrary.MakeTransform` _returnvalue_2))
        (elif (== (mod _index (`self.ConnectRate`)) 0)
          (`InstancedStaticMeshComponent.AddInstance` (`self.LadderConnect`) (`KismetMathLibrary.MakeTransform` _returnvalue_2))
          (else
            (`InstancedStaticMeshComponent.AddInstance` (`self.LadderMiddle`) (`KismetMathLibrary.MakeTransform` _returnvalue_2)))))))
  (bind _z (.z _returnvalue_2))
  (`SceneComponent.K2_SetRelativeLocation` (`self.EndPosition`) (`KismetMathLibrary.MakeVector` _finallocation_x _finallocation_y (+ _finallocation_z _z)) false false)
  (`SceneComponent.K2_SetRelativeLocationAndRotation` :`self` (`self.StartPositionUp`) :`NewLocation` (`KismetMathLibrary.MakeVector` 0.0 75.0 _z))
  (`SceneComponent.K2_SetRelativeLocation` (`self.TopCollision`) (`KismetMathLibrary.MakeVector` 0.0 40.0 (+ _z 150.0)) false false)
  (`SceneComponent.K2_SetRelativeLocation` (`self.Interaction`) (`KismetMathLibrary.MakeVector` 0.0 10.0 (- (* (`self.LadderStep`) 20.0) 15.0)) false false)
  (`BoxComponent.SetBoxExtent` (`self.Interaction`) (`KismetMathLibrary.MakeVector` 38.0 8.0 (+ (* (`self.LadderStep`) 20.0) 5.0)) true)
  (`SceneComponent.K2_SetRelativeLocation` (`self.ReleaseHeight`) (`KismetMathLibrary.MakeVector` 0.0 30.0 (`self.Release Height`)) false false))