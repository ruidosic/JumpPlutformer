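; Level chunk actor that builds a Length by Width grid of spawned element actors on BeginPlay.
; Spawn mode either places elements at the set spacing or starts them packed together at a raised or lowered height, recording each start point.
; A box collision is centered and sized from the grid dimensions.
; In the non-default modes, each element's ChunkMove then sends it to its spaced grid slot, optionally looping.
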(event `self.ReceiveBeginPlay`
  (`self.Setup`)
  (`self.ChunkInitialMove`))

(fn `CalculateChunkLength`
  (returns (ReturnValue :type "Float (double-precision)"))
  (return (+ (* (`self.Length`) (.x (`/Game/Blueprints/BP_ChunkElementBase.ElementSize` (`|GetArrayItem` (`self.ElementsRef`))))) (* (- (`self.Length`) 1) (`self.DistanceBetween`)))))

(fn `CalculateChunkWidth`
  (returns (ReturnValue :type "Float (double-precision)"))
  (return (+ (* (`self.Width`) (.y (`/Game/Blueprints/BP_ChunkElementBase.ElementSize` (`|GetArrayItem` (`self.ElementsRef`))))) (* (- (`self.Width`) 1) (`self.DistanceBetween`)))))

(fn `ChunkInitialMove`
  (bind _width (`self.Width`))
  (bind ((`ChunkMoveRateMultiplier_10_7EA243C7443330586C85F6B888EDE723` _chunkmoveratemultiplier) (`LoopMove?_14_DFABDB074D189FCBB35C0A993B6BE74B` _loopmove_)) (break `/Game/Blueprints/Struct_ChunkMove` (`self.Struct_ChunkMove`)))
  (if (not (`|EnumEquality` (`.SpawnMode_2_E955FC6D4D9AFD9BA0CBABB043D704A0` (break `/Game/Blueprints/Struct_ChunkMove` (`self.Struct_ChunkMove`))) "NewEnumerator0"))
    (for (_array_element _array_index) (`self.ElementsRef`)
      (`/Game/Blueprints/BP_ChunkElementBase.ChunkMove` _array_element (+ (`KismetMathLibrary.MakeVector` (* (/ _array_index _width) (.x (+ (`/Game/Blueprints/BP_ChunkElementBase.ElementSize` _array_element) (`self.DistanceBetween`)))) (* (mod _array_index _width) (.y (+ (`/Game/Blueprints/BP_ChunkElementBase.ElementSize` _array_element) (`self.DistanceBetween`))))) (`SceneComponent.K2_GetComponentLocation` (`self.DefaultSceneRoot`))) _chunkmoveratemultiplier _loopmove_))))

(fn `Setup`
  (locals (DeltaX :type "Float (double-precision)" :default 1.0))
  (bind ((`SpawnMode_2_E955FC6D4D9AFD9BA0CBABB043D704A0` _spawnmode) (`DownStartPoint_11_2E40272645E35B513F455E8F310B4497` _downstartpoint) (`UpStartPoint_12_B6BDE89847C0C65F8F9CA2BF0A39EDF5` _upstartpoint)) (break `/Game/Blueprints/Struct_ChunkMove` (`self.Struct_ChunkMove`)))
  (for _index (range (`self.Length`))
    (for _index_2 (range (`self.Width`))
      (bind _returnvalue (`|SpawnActorFromClass` (`self.ElementsClass`) (`KismetMathLibrary.MakeTransform` (0.0 0.0 0.0)) "Undefined" "OverrideRootScale" self (`self.ShuffleSides?`) null))
      (`KismetArrayLibrary.Array_Add` (`self.ElementsRef`) _returnvalue)
      (bind _elementsize (`/Game/Blueprints/BP_ChunkElementBase.ElementSize` _returnvalue))
      (bind _returnvalue_2 (- (+ (`SceneComponent.K2_GetComponentLocation` (`self.DefaultSceneRoot`)) (`KismetMathLibrary.MakeVector` (* _index (.x (+ _elementsize (select `/Game/Blueprints/Enum_SpawnMode` (`.SpawnMode_2_E955FC6D4D9AFD9BA0CBABB043D704A0` (break `/Game/Blueprints/Struct_ChunkMove` (`self.Struct_ChunkMove`))) :`NewEnumerator0` (`self.DistanceBetween`))))) (* _index_2 (.y (+ _elementsize (select `/Game/Blueprints/Enum_SpawnMode` (`.SpawnMode_2_E955FC6D4D9AFD9BA0CBABB043D704A0` (break `/Game/Blueprints/Struct_ChunkMove` (`self.Struct_ChunkMove`))) :`NewEnumerator0` (`self.DistanceBetween`))))) (select `/Game/Blueprints/Enum_SpawnMode` _spawnmode :`NewEnumerator1` _downstartpoint :`NewEnumerator2` _upstartpoint))) (`KismetMathLibrary.MakeVector` 0.0 0.0 (.z _elementsize))))
      (`KismetArrayLibrary.Array_Add` (`self.SpawnStartPoints`) _returnvalue_2)
      (`self.K2_SetActorLocation` _returnvalue _returnvalue_2 false false)
      (`SceneComponent.K2_SetWorldLocation` (`self.ChunkCollision`) (- (+ (`SceneComponent.K2_GetComponentLocation` (`self.DefaultSceneRoot`)) (`KismetMathLibrary.MakeVector` (/ (`self.CalculateChunkLength`) 2.0) (/ (`self.CalculateChunkWidth`) 2.0))) (`/Game/Blueprints/BP_ChunkElementBase.GetStaticMeshHalfSize` (`|GetArrayItem` (`self.ElementsRef`)))) false false)
      (`BoxComponent.SetBoxExtent` (`self.ChunkCollision`) (* (`KismetMathLibrary.MakeVector` (/ (`self.CalculateChunkLength`) 2.0) (/ (`self.CalculateChunkWidth`) 2.0) (`self.ChunkCollisionHeight`)) (`self.CunkCollisionMultiplier`)) true))))

(fn `UserConstructionScript`)