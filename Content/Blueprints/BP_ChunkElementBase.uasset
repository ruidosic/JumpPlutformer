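; Base actor for a chunk element: a movable platform piece that notifies overlapping actors for jump and platform detection.
; Construction sizes and offsets the JumpTrigger and PlatformDetect boxes from mesh bounds, optionally shuffling mesh rotation in 90-degree steps.
; ChunkMove uses timelines to lerp from the current location toward a target, optionally looping back and forth.
; Jump trigger exit and platform detect enter/exit send messages to the other actor.
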(event `self.JumpTrigger.OnComponentEndOverlap`
  (params (OverlappedComponent :type "PrimitiveComponent Object Reference") (OtherActor :type "Actor Object Reference") (OtherComp :type "PrimitiveComponent Object Reference") (OtherBodyIndex :type Integer))
  (message `/Game/Blueprints/BPI_CharacterMovement.JumpEvent` OtherActor))

(event `self.PlatformDetect.OnComponentBeginOverlap`
  (params (OverlappedComponent :type "PrimitiveComponent Object Reference") (OtherActor :type "Actor Object Reference") (OtherComp :type "PrimitiveComponent Object Reference") (OtherBodyIndex :type Integer) (bFromSweep :type Boolean) (SweepResult :type "HitResult Structure (by ref)"))
  (message `/Game/Blueprints/BPI_Platform.BeginOverlap` OtherActor))

(event `self.PlatformDetect.OnComponentEndOverlap`
  (params (OverlappedComponent :type "PrimitiveComponent Object Reference") (OtherActor :type "Actor Object Reference") (OtherComp :type "PrimitiveComponent Object Reference") (OtherBodyIndex :type Integer))
  (message `/Game/Blueprints/BPI_Platform.EndOverlap` OtherActor))

(event `/Game/Blueprints/BPI_Platform.BeginOverlap`)

(event `/Game/Blueprints/BPI_Platform.EndOverlap`)

(event `ChunkMove`
  (params (TargetPoint :type "Vector Structure") (NewRate :type "Float (double-precision)") (Loop :type Boolean))
  (set `self.InitialLocation` (`self.K2_GetActorLocation`))
  (`TimelineComponent.SetPlayRate` (`self.Initial Movement`) NewRate)
  (bind (_direction _alpha) (`Timeline|Initial Movement` :!via `PlayFromStart` :!label _label)
    (:`Update`
      (`self.K2_SetActorLocation` (`KismetMathLibrary.VLerp` (`self.K2_GetActorLocation`) TargetPoint (* _alpha (`GameplayStatics.GetWorldDeltaSeconds`)))))
    (:`Finished`
      (if Loop
        (bind (_direction_2 _alpha_2) (`Timeline|Timeline_0` :!via `PlayFromStart`)
          (:`Update`
            (`self.K2_SetActorLocation` (`KismetMathLibrary.VLerp` (`self.K2_GetActorLocation`) (`self.InitialLocation`) (* _alpha_2 (`GameplayStatics.GetWorldDeltaSeconds`)))))
          (:`Finished`
            (goto _label :!via `PlayFromStart`)))))))

(fn `DisableJumpTrigger`
  (`PrimitiveComponent.SetCollisionEnabled` (`self.JumpTrigger`) "QueryAndPhysics"))

(fn `EnableJumpTrigger`
  (`PrimitiveComponent.SetCollisionEnabled` (`self.JumpTrigger`) "NoCollision"))

(fn `GetStaticMeshHalfSize`
  (returns (Size :type "Vector Structure"))
  (return (`.BoxExtent` (`KismetMathLibrary.BreakBoxSphereBounds` (`StaticMesh.GetBounds` (`StaticMeshComponent.StaticMesh` (`self.ElementMesh`)))))))

(fn `ShuffleSide`
  (locals (Enum_RotationCoordinate :type "Array of /Game/Blueprints/Enum_RotationCoordinate Enum"))
  (bind _elementskeletalmesh (`self.ElementSkeletalMesh`))
  (if (`self.ShuffleSide?`)
    (`KismetArrayLibrary.Array_Shuffle` (`local.Enum_RotationCoordinate`))
    (for (_array_element _array_index) (`local.Enum_RotationCoordinate`)
      (switch `/Game/Blueprints/Enum_RotationCoordinate` _array_element
        (:`NewEnumerator0`
          (bind _returnvalue (* _array_index 90.0))
          (`SceneComponent.K2_AddRelativeRotation` _elementskeletalmesh (`KismetMathLibrary.MakeRotator` _returnvalue) false false)
          (`SceneComponent.K2_AddRelativeRotation` (`self.ElementMesh`) (`KismetMathLibrary.MakeRotator` _returnvalue) false false))
        (:`NewEnumerator1`
          (`SceneComponent.K2_AddRelativeRotation` _elementskeletalmesh (`KismetMathLibrary.MakeRotator` 0.0 _returnvalue) false false)
          (`SceneComponent.K2_AddRelativeRotation` (`self.ElementMesh`) (`KismetMathLibrary.MakeRotator` 0.0 _returnvalue) false false))
        (:`NewEnumerator2`
          (`SceneComponent.K2_AddRelativeRotation` _elementskeletalmesh (`KismetMathLibrary.MakeRotator` 0.0 0.0 _returnvalue) false false)
          (`SceneComponent.K2_AddRelativeRotation` (`self.ElementMesh`) (`KismetMathLibrary.MakeRotator` 0.0 0.0 _returnvalue) false false))))))

(fn `UserConstructionScript`
  (bind _jumptrigger (`self.JumpTrigger`))
  (bind _platformdetect (`self.PlatformDetect`))
  (bind _returnvalue (* (`self.GetStaticMeshHalfSize`) (`self.JumpTriggerSizeMultiplier`)))
  (bind _returnvalue_2 (`KismetMathLibrary.MakeVector` (.x (* (`self.GetStaticMeshHalfSize`) (`self.PlatformDetectSizeMultiplier`))) (.y (* (`self.GetStaticMeshHalfSize`) (`self.PlatformDetectSizeMultiplier`))) 200.0))
  (set `self.ElementSize` (* (`self.GetStaticMeshHalfSize`) 2))
  (`BoxComponent.SetBoxExtent` _jumptrigger _returnvalue true)
  (`SceneComponent.K2_AddLocalOffset` _jumptrigger (`KismetMathLibrary.MakeVector` 0.0 0.0 (.z _returnvalue)) false false)
  (`BoxComponent.SetBoxExtent` _platformdetect _returnvalue_2 true)
  (`SceneComponent.K2_AddLocalOffset` _platformdetect (`KismetMathLibrary.MakeVector` 0.0 0.0 (* -1 (.z _returnvalue_2))) false false)
  (`self.ShuffleSide`))