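; BP_CoreEngine is a core player-systems Blueprint that drives health, movement speed, footsteps, fall damage and camera focus for player 0, using defaults copied from CoreSettings.
; Damage clamps health, optionally preventing death on game events, then recalculates walk/run speed, which changes below 50 health.
; Sphere traces pick footstep and landing sounds by physical surface; landings also apply timer-measured fall damage.
; A focus timeline blends FOV and health-dependent depth-of-field aperture.
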(event `self.ReceiveBeginPlay`
  ;[1 1 1] Begin Play
  (`/Game/Blueprints/Core/BP_Functions.PlayerInput` true)
  (bind _output_get (set `self.PlayerCamera` (`|GetArrayItem` (`self.GetComponentsByTag` (`GameplayStatics.GetPlayerCharacter` 0) "/Script/Engine.CameraComponent" "Camera"))))
  (`CameraComponent.SetFieldOfView` _output_get (`self.DefaultFOV`)))

(event `GetDamage`
  (params (`Game Event` :type Boolean) (`Event Settings` :type "/Game/Blueprints/Events/Structs/Struct_GE_Damage Structure") (DamagePoint :type "Float (double-precision)"))
  (if (not (`self.Dead`))
    (`self.CalculateDamage` `Game Event` `Event Settings` DamagePoint)))

(event `CalculateDamage`
  (params (GameEvent :type Boolean) (EventSettings :type "/Game/Blueprints/Events/Structs/Struct_GE_Damage Structure") (DamagePoint :type "Float (double-precision)"))
  (bind _health (`self.Health`))
  (bind _returnvalue (- (`self.Health`) (select `bool` (< DamagePoint 0.0) :`false` DamagePoint :`true` (* DamagePoint -1.0))))
  (bind _output_get (set `self.Health` (`KismetMathLibrary.FClamp` _returnvalue (select `bool` (<= _returnvalue 0.0) :`true` (select `bool` (and GameEvent (`.ForcetoSurviveAfterThisDamage_5_43934569492BD4EF11B93583A9A726E9` (break `/Game/Blueprints/Events/Structs/Struct_GE_Damage` EventSettings))) :`true` (select `bool` (<= _health 10.0) :`false` 10.0 :`true` _health))) 100.0)))
  (`self.CalculateSpeed`)
  (`KismetSystemLibrary.PrintString` (`KismetStringLibrary.Conv_DoubleToString` _output_get)))

(event `StartFocus`
  (set `self.CurrentAperture` (`self.DOF Aperature`))
  (bind (_direction _alpha) (`Timeline|FocusTimeline` :!label _label)
    (:`Update`
      (set `self.Focusing` (>= _alpha 1.0))
      (bind _output_get (set `self.Current FOV` (`KismetMathLibrary.Lerp` (`self.DefaultFOV`) (`self.FocusFOV`) _alpha)))
      (`CameraComponent.SetFieldOfView` (`self.PlayerCamera`) _output_get)
      (set `self.DOF Aperature` (`KismetMathLibrary.Lerp` (`self.CurrentAperture`) (`KismetMathLibrary.MapRangeClamped` (`self.Health`) 50.0 0.0 1.0 20.0) _alpha)) ; Depend by health
    )))

(event `StopFocus`
  (`|ExecutionSequence`
    (:`then_0`
      (goto _label :!via `Stop`))
    (:`then_1`
      (goto _label :!via `SetNewTime`))))

(event `EndFocus`
  (goto _label :!via `Reverse`))

(fn `CalculateSpeed`
  (bind _walkspeed (`self.WalkSpeed`))
  (bind _runspeed (`self.RunSpeed`))
  (bind _returnvalue (/ _walkspeed 2.0))
  (bind _returnvalue_2 (/ _runspeed 2.0))
  ;[1 1 1] Recalculate Walk Speed, if Health < 50
  (set `self.LowHealthWalkSpeed` (`KismetMathLibrary.Lerp` _returnvalue (`KismetMathLibrary.MapRangeClamped` _returnvalue 0.0 _walkspeed _returnvalue 300.0) (/ (`self.Health`) 50.0)))
  (set `self.LowHealthRunSpeed` (`KismetMathLibrary.Lerp` _returnvalue_2 (`KismetMathLibrary.MapRangeClamped` _returnvalue_2 0.0 _runspeed _returnvalue_2 400.0) (/ (`self.Health`) 50.0)))
  (set `CharacterMovementComponent.MaxWalkSpeed` (select `bool` (`self.Running`) :`false` (select `bool` (< (`self.Health`) 50.0) :`false` (`self.WalkSpeed`) :`true` (`self.LowHealthWalkSpeed`)) :`true` (select `bool` (< (`self.Health`) 50.0) :`false` (`self.RunSpeed`) :`true` (`self.LowHealthRunSpeed`))) (`Character.CharacterMovement` (`GameplayStatics.GetPlayerCharacter` 0))))

(fn `ClearFallingTimer`
  (bind _fallingtimer (`self.FallingTimer`))
  (if (`KismetSystemLibrary.K2_IsValidTimerHandle` _fallingtimer)
    (`KismetSystemLibrary.K2_ClearAndInvalidateTimerHandle` _fallingtimer)
    (set `self.FallingDuration` 0.0)
    (set `self.FallingTimer` (struct))))

(fn `Falling`
  (if (`NavMovementComponent.IsFalling` (`Character.CharacterMovement` (`GameplayStatics.GetPlayerCharacter` 0)))
    (set `self.FallingDuration` (+ (`self.FallingDuration`) 0.1))))

(fn `FallingDamage`
  (if (`KismetMathLibrary.InRange_FloatFloat` (`self.FallingDuration`) 0.0 2.0)
    _
    (elif (`KismetMathLibrary.InRange_FloatFloat` (`self.FallingDuration`) 2.0 3.0 false)
      (`self.GetDamage` false (struct) (* (`self.FallingDuration`) (`self.FallingDamageMultiplier`)))
      (else
        (`self.GetDamage` false (struct) 100.0))))
  (`self.ClearFallingTimer`))

(fn `Footstep/Headshake`
  (params (FootstepType :type "/Game/Blueprints/Core/Enums/Enum_FootstepAction Enum" :default "NewEnumerator0"))
  (bind _returnvalue (`self.K2_GetActorLocation` (`GameplayStatics.GetPlayerPawn` 0)))
  (bind _returnvalue_2 (`Pawn.GetMovementComponent` (`GameplayStatics.GetPlayerPawn` 0)))
  (bind _returnvalue_3 (`self.K2_GetActorLocation` (`GameplayStatics.GetPlayerPawn` 0)))
  (bind ((`CarpetJump_24_9B4DB1BA46AC9D2C5194EFAD9F7DDD2E` _carpetjump) (`DirtJump_26_DA5900BE47345EEDB90E9AA91B8A1E38` _dirtjump) (`GrassJump_28_5B0465E449254873000502896F74E9E6` _grassjump) (`MetalJump_36_EB2AF65F4F2B5DD665C1E2A1ADFB3EAD` _metaljump) (`RockJump_38_C4F2DB5540BADC665285CD92F0A88453` _rockjump) (`ConcreteJump_41_BB33FA604D683FB8299812A50BF20ED6` _concretejump) (`WoodJump_45_F1023510426713EC8984288FE949D6C1` _woodjump) (`GravelJump_52_541B44654E1838DED8A56AAF820A11B7` _graveljump) (`GroundJump_54_FFE270784EF94A776E9567A7268D3568` _groundjump) (`PlasticJump_57_6E538EA04FE1D0970DD4AC8CBAA5FC2E` _plasticjump) (`SandJump_61_012E829F444747C8BCB839BFB4953CEF` _sandjump) (`SnowJump_68_E21DE28C4B7256FF60255AB50DBCA429` _snowjump) (`WaterJump_70_452AB0BA449F584996DC9DB08FC3E361` _waterjump)) (break `/Game/Blueprints/Core/Structs/Struct_FootstepSettings` (`.FootstepSettings_9_F5CFEE304A26BB76A4886D9A17B501EF` (break `/Game/Blueprints/Core/Structs/Struct_CoreSettings` (`self.CoreSettings`)))))
  (bind ((`Carpet_23_BB90B1654C607E3E8BB1E1A47DAF852E` _carpet) (`Dirt_25_718262CC417BAE47A127F584C80EAD45` _dirt) (`Grass_27_9A4942ED4C2C6ECB61479EA2CD492DAE` _grass) (`Metal_35_1425726C4702E3B8A94FEF8F1DFDC872` _metal) (`Rock_37_6C050E2F441FF86E97D7F5AE6C51C024` _rock) (`Concrete_39_A9DA95764EF0009AC6AED5B9C3E7E738` _concrete) (`Wood_42_4EC6C5B94C41A45136AE05A3DB09434D` _wood) (`Gravel_51_2C732894440C4A0C962BEEAE22BF65EA` _gravel) (`Ground_53_48AD0C074E6DE3D402787D8BA3CC6511` _ground) (`Plastic_55_4BCCA0B7467C2070C621EFB3169FDAB7` _plastic) (`Sand_59_A3E28827488DA3CFF081D1BCA483EE61` _sand) (`Snow_66_1EFA29064E96023F2D73949DA304DE0B` _snow) (`Water_69_6503DBBB46E94D4CFBB282B64DD4AA40` _water)) (break `/Game/Blueprints/Core/Structs/Struct_FootstepSettings` (`.FootstepSettings_9_F5CFEE304A26BB76A4886D9A17B501EF` (break `/Game/Blueprints/Core/Structs/Struct_CoreSettings` (`self.CoreSettings`)))))
  (switch `/Game/Blueprints/Core/Enums/Enum_FootstepAction` FootstepType
    (:`NewEnumerator0`
      (if (and (`NavMovementComponent.IsMovingOnGround` _returnvalue_2) (>= (`KismetMathLibrary.VSize` (`MovementComponent.Velocity` _returnvalue_2)) 50.0) (`self.HeadShakeEnabled`))
        (`PlayerController.ClientStartCameraShake` :`self` (`GameplayStatics.GetPlayerController` 0) :`Shake` "/Game/Blueprints/Core/CameraShakes/HeadShakeWalking.HeadShakeWalking_C" :`Scale` (* (/ (`CharacterMovementComponent.MaxWalkSpeed` (`Character.CharacterMovement` (`GameplayStatics.GetPlayerCharacter` 0))) 100.0) (`self.HeadShakeValue`)))
        (if (and (> (`KismetMathLibrary.VSize` (- (`self.K2_GetActorLocation` (`GameplayStatics.GetPlayerPawn` 0)) (`self.CurrentFootLocation`))) (`self.StepSize`)) (`NavMovementComponent.IsMovingOnGround` (`Pawn.GetMovementComponent` (`GameplayStatics.GetPlayerPawn` 0))))
          (bind _outactors (`GameplayStatics.GetAllActorsWithTag` "IgnoreTrace"))
          (bind (_outhit _returnvalue_4) (`KismetSystemLibrary.SphereTraceSingle` _returnvalue_3 (- _returnvalue_3 (0.0 0.0 100.0)) 30.0 "TraceTypeQuery1" true _outactors))
          (if _returnvalue_4
            (bind (_bblockinghit _binitialoverlap _time _distance _location _impactpoint _normal _impactnormal _physmat) (`GameplayStatics.BreakHitResult` _outhit))
            (`GameplayStatics.SpawnSoundAtLocation` (select `EPhysicalSurface` (`PhysicalMaterial.SurfaceType` _physmat) :`SurfaceType_Default` _ground :`SurfaceType1` _carpet :`SurfaceType2` _dirt :`SurfaceType3` _grass :`SurfaceType4` _metal :`SurfaceType5` _rock :`SurfaceType6` _concrete :`SurfaceType7` _wood :`SurfaceType8` _gravel :`SurfaceType9` _ground :`SurfaceType10` _plastic :`SurfaceType11` _sand :`SurfaceType12` _snow :`SurfaceType13` _water) _location (struct) 1.0 1.0 0.0 null null)
            (set `self.CurrentFootLocation` _location)))))
    (:`NewEnumerator1`
      ;[1 1 1] Ignore Tag for all trace
      (bind _outactors_2 (`GameplayStatics.GetAllActorsWithTag` "IgnoreTrace"))
      (bind (_outhit_2 _returnvalue_5) (`KismetSystemLibrary.SphereTraceSingle` _returnvalue (- _returnvalue (0.0 0.0 100.0)) 30.0 "TraceTypeQuery1" true _outactors_2))
      (if _returnvalue_5
        (bind (_bblockinghit_2 _binitialoverlap_2 _time_2 _distance_2 _location_2 _impactpoint_2 _normal_2 _impactnormal_2 _physmat_2) (`GameplayStatics.BreakHitResult` _outhit_2))
        (`GameplayStatics.SpawnSoundAtLocation` (select `EPhysicalSurface` (`PhysicalMaterial.SurfaceType` _physmat_2) :`SurfaceType_Default` _groundjump :`SurfaceType1` _carpetjump :`SurfaceType2` _dirtjump :`SurfaceType3` _grassjump :`SurfaceType4` _metaljump :`SurfaceType5` _rockjump :`SurfaceType6` _concretejump :`SurfaceType7` _woodjump :`SurfaceType8` _graveljump :`SurfaceType9` _groundjump :`SurfaceType10` _plasticjump :`SurfaceType11` _sandjump :`SurfaceType12` _snowjump :`SurfaceType13` _waterjump) _location_2 (struct) 1.0 1.0 0.0 null null)
        (`self.FallingDamage`)
        (if (`self.HeadShakeEnabled`)
          (`PlayerController.ClientStartCameraShake` :`self` (`GameplayStatics.GetPlayerController` 0) :`Shake` "/Game/Blueprints/Core/CameraShakes/HeadShakeLanded.HeadShakeLanded_C" :`Scale` 10.0))))))

(fn `StartFallingTimer`
  (bind _returnvalue (`KismetSystemLibrary.K2_SetTimer` null "Falling" 0.1 true))
  (set `self.FallingTimer` _returnvalue))

(fn `UserConstructionScript`
  (`self.DefaultSettimgs`))