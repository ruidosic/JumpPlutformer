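; Base map chunk element: a platform that can move to a target, optionally looping, and falls and destroys itself shortly after its jump trigger is overlapped.
; Construction sizes both trigger boxes from mesh bounds and can shuffle 90-degree mesh rotations.
; The downward detection box messages overlapped actors, letting elements switch off their jump triggers while covered.
; Timelines drive movement, and leaving the jump trigger sends a jump message to that actor.
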(fn `DestroyEffect`
  (`GameplayStatics.SpawnEmitterAtLocation` "/Game/Assets/VFX/P_SimpleGem.P_SimpleGem" (`KismetMathLibrary.MakeVector` (.x (`SceneComponent.K2_GetComponentLocation` (`self.DefaultSceneRoot`))) (.y (`SceneComponent.K2_GetComponentLocation` (`self.DefaultSceneRoot`))) (+ (.z (`SceneComponent.K2_GetComponentLocation` (`self.DefaultSceneRoot`))) (/ (.z (`self.ElementSize`)) 1.0)))))

(fn `DisableJumpTrigger`
  (`PrimitiveComponent.SetCollisionEnabled` (`self.JumpTrigger`) "NoCollision"))

(fn `EnableJumpTrigger`
  (`PrimitiveComponent.SetCollisionEnabled` (`self.JumpTrigger`) "QueryOnly"))

(fn `GetStaticMeshHalfSize`
  (returns (Size :type "Vector Structure"))
  (return (`.BoxExtent` (`KismetMathLibrary.BreakBoxSphereBounds` (`StaticMesh.GetBounds` (`StaticMeshComponent.StaticMesh` (`self.ElementMesh`)))))))

(fn `ShuffleSide`
  (locals (Enum_RotationCoordinate :type "Array of /Game/Blueprints/Map/Enum_RotationCoordinate Enum"))
  (bind _elementskeletalmesh (`self.ElementSkeletalMesh`))
  (if (`self.ShuffleSide?`)
    (`KismetArrayLibrary.Array_Shuffle` (`local.Enum_RotationCoordinate`))
    (for (_array_element _array_index) (`local.Enum_RotationCoordinate`)
      (switch `/Game/Blueprints/Map/Enum_RotationCoordinate` _array_element
        (:`NewEnumerator0`
          (bind _returnvalue (* _array_index 90.0))
          (`SceneComponent.K2_AddRelativeRotation` _elementskeletalmesh (`KismetMathLibrary.MakeRotator` _returnvalue) false false)
          (`SceneComponent.K2_AddRelativeRotation` (`self.ElementMesh`) (`KismetMathLibrary.MakeRotator` _returnvalue) false false))
        (:`NewEnumerator1`
          (`SceneComponent.K2_AddRelativeRotation` _elementskeletalmesh (`KismetMathLibrary.MakeRotator` 0.0 _returnvalue) false false)
          (`SceneComponent.K2_AddRelativeRotation` (`self.ElementMesh`) (`KismetMathLibrary.MakeRotator` 0.0 _returnvalue) false false))
        (:`NewEnumerator2`
          (`SceneComponent.K2_AddRelativeRotation` _elementskeletalmesh (`KismetMathLibrary.MakeRotator` 0.0 0.0 _returnvalue) false false)
          (`SceneComponent.K2_AddRelativeRotation` (`self.ElementMesh`) (`KismetMathLibrary.MakeRotator` 0.0 0.0 _returnvalue) false false))))))

(fn `UserConstructionScript`
  (bind _jumptrigger (`self.JumpTrigger`))
  (bind _platformdetect (`self.PlatformDetect`))
  (bind _returnvalue (* (`self.GetStaticMeshHalfSize`) (`self.JumpTriggerSizeMultiplier`)))
  (bind _returnvalue_2 (`KismetMathLibrary.MakeVector` (.x (* (`self.GetStaticMeshHalfSize`) (`self.PlatformDetectSizeMultiplier`))) (.y (* (`self.GetStaticMeshHalfSize`) (`self.PlatformDetectSizeMultiplier`))) 200.0))
  (set `self.ElementSize` (* (`self.GetStaticMeshHalfSize`) 2))
  (`BoxComponent.SetBoxExtent` _jumptrigger _returnvalue true)
  (`SceneComponent.K2_AddLocalOffset` _jumptrigger (`KismetMathLibrary.MakeVector` 0.0 0.0 (.z _returnvalue)) false false)
  (`BoxComponent.SetBoxExtent` _platformdetect _returnvalue_2 true)
  (`SceneComponent.K2_AddLocalOffset` _platformdetect (`KismetMathLibrary.MakeVector` 0.0 0.0 (* -1 (.z _returnvalue_2))) false false)
  (`self.ShuffleSide`))