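; BP_Use is an interactable actor with empty Use, AlternativeUse, Open/On and Close/Off functions, apparently a base for usable objects.
; GameEventCheck increments counters on GameEvents entries matching the given interaction and caches those reaching their AfterNTimes threshold, resetting counters not marked DoOnce.
; It then spawns a BP_GameEvents actor to run each cached event.
; ControllerInput toggles the actor's input from player controller 0.
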(fn `AlternativeUse`
  (params (GameEvent :type Boolean)))

(fn `Close/Off`
  (params (GameEvent :type Boolean)))

(fn `ControllerInput`
  (params (Enabled :type Boolean))
  (bind _returnvalue (`GameplayStatics.GetPlayerController` 0))
  (if Enabled
    (`self.EnableInput` _returnvalue)
    (else
      (`self.DisableInput` _returnvalue))))

(fn `GameEventCheck`
  (params (Check :type "/Game/Blueprints/Events/Enums/Enum_GameEventCheck Enum" :default "NewEnumerator0"))
  (for (_array_element _array_index) (`self.GameEvents`)
    (bind (_triggerinteraction _afterntimes _counter _doonce) (break `/Game/Blueprints/Events/Structs/Struct_GameEvents` _array_element))
    (if (`|EnumEquality` _triggerinteraction Check)
      (bind _structout (setmembers `/Game/Blueprints/Events/Structs/Struct_GameEvents` :`StructRef` _array_element :`Counter` (+ _counter 1)))
      (`KismetArrayLibrary.Array_Set` (`self.GameEvents`) _array_index _structout)
      (bind (_triggerinteraction_2 _afterntimes_2 _counter_2) (break `/Game/Blueprints/Events/Structs/Struct_GameEvents` _array_element))
      (if (== _afterntimes_2 _counter_2)
        (`KismetArrayLibrary.Array_Add` (`self.IndexCache`) _array_index)
        (if (not _doonce)
          ;[1 1 1] Reset Counter
          (bind _structout_2 (setmembers `/Game/Blueprints/Events/Structs/Struct_GameEvents` :`StructRef` _array_element :`Counter` 0))
          (`KismetArrayLibrary.Array_Set` (`self.GameEvents`) _array_index _structout_2)))))
  ;[1 1 1] Do Game Events
  (for _array_element_2 (`self.IndexCache`)
    (bind _returnvalue (`|SpawnActorFromClass` "/Game/Blueprints/Events/BP_GameEvents.BP_GameEvents_C" (`KismetMathLibrary.MakeTransform` (0.0 0.0 0.0)) "DontSpawnIfColliding" "OverrideRootScale" null null))
    (`/Game/Blueprints/Events/BP_GameEvents.GameEvent` _returnvalue (`.GameEvent_13_AD15CCB942DB8106E33568858C6CF317` (break `/Game/Blueprints/Events/Structs/Struct_GameEvents` (`|GetArrayItem` (`self.GameEvents`) _array_element_2))))))

(fn `Open/On`
  (params (GameEvent :type Boolean)))

(fn `Use`
  (params (GameEvent :type Boolean)))

(fn `UserConstructionScript`)