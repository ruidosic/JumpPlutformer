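; Event trigger volume that runs a game event check when the player pawn stays inside its box for a configurable duration.
; Begin overlap restarts a timeline whose event track calls the check with a fixed enum value, and end overlap stops it.
; The construction script creates the game events, sizes and offsets the box so the billboard sits at its corner, and sets the timeline's play rate from the duration.
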(event `self.OverlapTrigger.OnComponentBeginOverlap`
  (params (OverlappedComponent :type "PrimitiveComponent Object Reference") (OtherActor :type "Actor Object Reference") (OtherComp :type "PrimitiveComponent Object Reference") (OtherBodyIndex :type Integer) (bFromSweep :type Boolean) (SweepResult :type "HitResult Structure (by ref)"))
  (if (== OtherActor (`GameplayStatics.GetPlayerPawn` 0))
    (`Timeline|TriggerTimeline` :!via `PlayFromStart` :!label _label
      (:`Event`
        (`self.GameEventCheck` "NewEnumerator7")))))

(event `self.OverlapTrigger.OnComponentEndOverlap`
  (params (OverlappedComponent :type "PrimitiveComponent Object Reference") (OtherActor :type "Actor Object Reference") (OtherComp :type "PrimitiveComponent Object Reference") (OtherBodyIndex :type Integer))
  (if (== OtherActor (`GameplayStatics.GetPlayerPawn` 0))
    (goto _label :!via `Stop`)))

(fn `UserConstructionScript`
  (set `self.GameEvents` (`self.CreateGameEvents`))
  (`BoxComponent.SetBoxExtent` (`self.OverlapTrigger`) (`self.TriggerBoxExtend`) true)
  (`SceneComponent.K2_SetRelativeLocation` (`self.OverlapTrigger`) (`self.TriggerBoxExtend`) false false) ; for billboard "Angle" Location in Trigger
  (`/Game/Blueprints/Core/BP_Functions.PlayRate` (`self.TriggerTimeline`) (`self.OverlapDuration(Sec)`)))