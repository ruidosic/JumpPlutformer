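; Trigger box that unlocks when the required set of specific or tagged actors is placed inside it, raising game events.
; CheckActors filters overlaps against the required actor list and tag list, and a counter tracks matches entering and leaving.
; Reaching the combined required count clears Locked and fires one event; exits while unlocked fire another, without relocking.
; The construction script sizes the box from TriggerSettings and initializes the events.
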(event `self.PutTrigger.OnComponentBeginOverlap`
  (params (OverlappedComponent :type "PrimitiveComponent Object Reference") (OtherActor :type "Actor Object Reference") (OtherComp :type "PrimitiveComponent Object Reference") (OtherBodyIndex :type Integer) (bFromSweep :type Boolean) (SweepResult :type "HitResult Structure (by ref)"))
  ;[1 1 1] Overlap
  (`self.CheckActors` OtherActor)
  (`/Engine/EditorBlueprintResources/StandardMacros.IncrementInt` (`self.Counter`)
    (:`  `
      (if (== (`self.Counter`) (+ (`KismetArrayLibrary.Array_Length` (`self.Required Actor(s) for Unlock`)) (`self.Required Number Of Tagged Actor(s)`)))
        (set `self.Locked` false)
        (`self.GameEventCheck` "NewEnumerator9")))))

(event `self.PutTrigger.OnComponentEndOverlap`
  (params (OverlappedComponent :type "PrimitiveComponent Object Reference") (OtherActor :type "Actor Object Reference") (OtherComp :type "PrimitiveComponent Object Reference") (OtherBodyIndex :type Integer))
  ;[1 1 1] Overlap
  (`self.CheckActors` OtherActor)
  (`/Engine/EditorBlueprintResources/StandardMacros.DecrementInt` (`self.Counter`)
    (:`  `
      (if (not (`self.Locked`))
        (`self.GameEventCheck` "NewEnumerator8")))))

(fn `UserConstructionScript`
  (`BoxComponent.SetBoxExtent` (`self.PutTrigger`) (`.TriggerSize_6_EDD3540D42C23AAC2C75829805BF9043` (break `/Game/Blueprints/UsableAssets/Doors/Structs/Struct_TriggerSettings` (`self.TriggerSettings`))) true)
  (set `self.GameEvents` (`self.CreateGameEvents`)))