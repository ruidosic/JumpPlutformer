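; BP_GameEvents is a spawnable actor that executes data-driven environment and sound events from GameEvent structs.
; Batch events spawn a fresh BP_GameEvents per array entry, giving most entries independent delays and state.
; Workers handle repeatable interactions, timeline-lerped transform sequences, tagged actor spawning with optional attachment, hide/destroy and 2D sound.
; The hide batch spawns actors without calling its worker, and the 3D sound handler is empty.
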(fn `UserConstructionScript`)