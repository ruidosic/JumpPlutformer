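; BP_JumpTrigger is a box trigger event Blueprint that tells actors overlapping it to jump with a set Z velocity.
; A flag picks begin or end overlap as the cue; after a configurable delay it sends the actor a jump message, then runs a game event check.
; The construction script sizes the box and offsets it by its extent, placing a corner at its parent's origin, and creates the game events list.
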(event `self.Trigger.OnComponentBeginOverlap`
  (params (OverlappedComponent :type "PrimitiveComponent Object Reference") (OtherActor :type "Actor Object Reference") (OtherComp :type "PrimitiveComponent Object Reference") (OtherBodyIndex :type Integer) (bFromSweep :type Boolean) (SweepResult :type "HitResult Structure (by ref)"))
  ;[1 1 1] JumpEvent On Begin Overlap
  (if (not (`self.JumpOnEndOverlap`))
    (`self.Jump Event` OtherActor)))

(event `self.Trigger.OnComponentEndOverlap`
  (params (OverlappedComponent :type "PrimitiveComponent Object Reference") (OtherActor :type "Actor Object Reference") (OtherComp :type "PrimitiveComponent Object Reference") (OtherBodyIndex :type Integer))
  ;[1 1 1] JumpEvent On End Overlap
  (if (`self.JumpOnEndOverlap`)
    (`self.Jump Event` OtherActor)))

(event `Jump Event`
  (params (Actor :type "Actor Object Reference"))
  ;[1 1 1] Jump Event
  (`KismetSystemLibrary.Delay` (`self.DelayBeforeJump`))
  (message `PortalInterface.JumpEvent` Actor (`self.JumpZVelocity`))
  (`self.GameEventCheck` "NewEnumerator6"))

(fn `UserConstructionScript`
  (`parent.UserConstructionScript`)
  (`BoxComponent.SetBoxExtent` (`self.Trigger`) (`self.BoxExtended`) true)
  (`SceneComponent.K2_SetRelativeLocation` (`self.Trigger`) (`self.BoxExtended`) false false)
  (set `self.GameEvents` (`self.CreateGameEvents`)))